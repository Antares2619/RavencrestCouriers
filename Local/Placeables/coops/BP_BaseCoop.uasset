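; Base bird coop placeable that houses bird items and lets players send item messages to other destinations by messenger bird.
; Interaction checks container access, then opens the crafting GUI, whose send and receive-toggle signals feed the messaging endpoint component.
; PetInventory, capped at MaxBirds, drives nest meshes, idle animations and per-type transforms after a random delay, with extra handling for bats.
; Closing the UI requests a rename when a custom name exists.
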(event Custom|ClientBindUI
  (params (destinations :type Array%20of%20Strings))
  ;[1 1 1] Open the Coop Messaging UI
  (bind _windowroot (|GUIModuleControllerActivate (Class|GUIModuleController|GetGUIModuleController) (Utilities|Name|MakeLiteralName "RACO_BirdCoop_CraftingGUI") true false) ; Testing different approach for empty dest list issue
    (:OnActivate
      (bind _asw_raco_bird_coop_crafting_gui (Utilities|Casting|CastToW_RACO_BirdCoop_CraftingGUI _windowroot))
      (Default|InitMessagingUI _asw_raco_bird_coop_crafting_gui destinations (Variables|/Game/Mods/RavencrestCouriers/System/BP_RACO_MessagingEndpoint_AC.BP_RACO_MessagingEndpoint_AC_C|GetcanReceive (Variables|Default|GetBP_RACO_MessagingEndpoint_AC)))
      (EventDispatchers|BindEventtoSignalSendMessage _asw_raco_bird_coop_crafting_gui (delegate Custom|OnSignalSendMessage))
      (EventDispatchers|BindEventtoSignalToggleCanReceive _asw_raco_bird_coop_crafting_gui (delegate Custom|OnSignalToggleCanReceive))
      (EventDispatchers|BindEventtoSignalMessengerBirdChanged _asw_raco_bird_coop_crafting_gui (delegate Custom|OnSignalMessengerBirdChanged))
      (EventDispatchers|BindEventtoSignalClosing _asw_raco_bird_coop_crafting_gui (delegate Custom|OnUIClosing)))))

(event Custom|receiveMessengerBirdProfile
  (params (birdProfile :type STRUCT%20RACO%20Bird%20Profile%20Structure))
  ;[1 1 1] Open the Coop Messaging UI
  (Default|HandleMessengerBirdProfile (stale Custom|ClientBindUI _asw_raco_bird_coop_crafting_gui) birdProfile))

(event Custom|OnSignalToggleCanReceive
  (params (canReceive :type Boolean))
  ;[1 1 1] Open the Coop Messaging UI
  (Default|DoToggleCanReceive (Variables|Default|GetBP_RACO_MessagingEndpoint_AC) canReceive))

(event Custom|OnUIClosing
  (params (window :type Window%20Root%20Object%20Reference))
  ;[1 1 1] Open the Coop Messaging UI
  (CallFunction|UpdateBuildableName))

(event Custom|OnSignalMessageSent
  (params (accepted :type Boolean) (errorMessage :type String) (messageRequest :type STRUCT%20RACO%20Message%20in%20Flight%20Structure))
  ;[1 1 1] Open the Coop Messaging UI
  (EventDispatchers|UnbindEventfromSignalMessageSent (Variables|Default|GetBP_RACO_MessagingEndpoint_AC) (delegate Custom|OnSignalMessageSent))
  (Default|HandleMessageFeedback (stale Custom|ClientBindUI _asw_raco_bird_coop_crafting_gui) accepted errorMessage messageRequest))

(event Custom|HandlePetInventoryChanged
  (params (index :type Integer) (item :type Game%20Item%20Object%20Reference) (srcInventory :type Item%20Inventory%20Object%20Reference) (srcIndex :type Integer))
  ;[1 1 1] Handle bird animations
  (Utilities|FlowControl|Delay (Math|Random|RandomFloatinRange 0.0 1.0))
  (CallFunction|UpdateBirdAnimations))

(event Custom|OnSignalMessengerBirdChanged
  (params (messengerBird :type Game%20Item%20Ref%20Structure))
  ;[1 1 1] Open the Coop Messaging UI
  (CallFunction|ResolveMessengerBirdProfile messengerBird))

(event Custom|HandlePetInventoryChanged2
  ;[1 1 1] Handle bird animations
  (Utilities|FlowControl|Delay (Math|Random|RandomFloatinRange 0.0 1.0))
  (CallFunction|UpdateBirdAnimations))

(event Custom|resolveMessengerBirdProfile
  (params (birdItemRef :type Game%20Item%20Ref%20Structure))
  ;[1 1 1] Open the Coop Messaging UI
  (bind _item (CallFunction|ResolveGameItemRef birdItemRef))
  (bind _asbp_base_bird_item (Utilities|Casting|CastToBP_BaseBirdItem _item))
  (CallFunction|ReceiveMessengerBirdProfile (Variables|/Game/Mods/RavencrestCouriers/Items/BP_BaseBirdItem.BP_BaseBirdItem_C|GetbirdProfile _asbp_base_bird_item)))

(event Custom|OnSignalSendMessage
  (params (carrier :type Game%20Item%20Ref%20Structure) (items :type Array%20of%20Game%20Item%20Ref%20Structures) (recipientID :type String))
  (bind _bp_raco_messagingendpoint_ac (Variables|Default|GetBP_RACO_MessagingEndpoint_AC))
  ;[1 1 1] Open the Coop Messaging UI
  (EventDispatchers|BindEventtoSignalMessageSent _bp_raco_messagingendpoint_ac (delegate Custom|OnSignalMessageSent))
  (Default|TrySendMessage _bp_raco_messagingendpoint_ac carrier items recipientID))

(event EventInteractableActivate
  (params (Component :type Primitive%20Component%20Object%20Reference) (Instigator :type Player%20Controller%20Object%20Reference) (HitIndex :type Integer) (TriggeredFromRadialWheel :type Boolean))
  ;[1 1 1] Access check
  (if (.CanAccess (Class|PlaceableBase|CanAccessContainer (Pawn|GetControlledPawn Instigator)))
    ;[1 1 1] Open the Coop Messaging UI
    (bind _destinations (Default|InitforMessagingUI (Variables|Default|GetBP_RACO_MessagingEndpoint_AC) Instigator (Utilities|Name|MakeLiteralName "RACO_BirdCoop_CraftingGUI") true))
    (CallFunction|ClientBindUI _destinations)))

(event EventBeginPlay
  (bind _petinventory (Variables|Default|GetPetInventory))
  (|CallParentFunction)
  (Utilities|FlowControl|Sequence
    (:then_0
      (Variables|/Game/Mods/RavencrestCouriers/System/BP_RACO_MessagingEndpoint_AC.BP_RACO_MessagingEndpoint_AC_C|SetaudioComponent (Variables|Default|GetBP_RACO_MessagingEndpoint_AC) (Variables|Default|GetBirdAudio))
      (CallFunction|CustomizePetSlots)
      (for (_array_element _array_index) (Variables|Default|GetPets)
        (Utilities|Array|SetArrayElem (Variables|Default|GetPetOriginalTransforms) _array_index (Transformation|GetRelativeTransform _array_element) true)))
    (:then_1
      ;[1 1 1] Handle bird animations
      (EventDispatchers|BindEventtoSignalItemAdded _petinventory (delegate Custom|HandlePetInventoryChanged))
      (EventDispatchers|BindEventtoSignalItemRemoved _petinventory (delegate Custom|HandlePetInventoryChanged))
      (EventDispatchers|BindEventtoSignalInventoryRecivedonClient _petinventory (delegate Custom|HandlePetInventoryChanged2)))
    (:then_2
      ;[1 1 1] Nest Size
      (Class|ItemInventory|SetMaxItemCount (Variables|Default|GetPetInventory) (Variables|Default|GetmaxBirds)))))

(fn ConstructionScript
  (|CallParentFunction))

(fn UpdateBuildableName
  (if (Class|BuildableBase|HasCustomBuildableName)
    (Default|ReqChangeName (Actor|GetComponentbyClass (Pawn|GetControlledPawn (Game|GetPlayerController 0)) "/Game/Mods/RavencrestCouriers/System/BP_RACO_AC.BP_RACO_AC_C") self (Class|BuildableBase|GetBuildableName false))))

(fn CustomizePetSlots)

(fn ClientGetCraftingGUICenterPanel
  (params (Instigator :type Player%20Controller%20Object%20Reference))
  (return (Utilities|Name|MakeLiteralName "BirdCoopInventory")))

(fn GetNestedBirds
  (bind _array_element (Utilities|ForEachLoopFast (Variables|/Script/ConanSandbox.ItemInventory|GetItemList (Variables|Default|GetPetInventory)))
    (:LoopBody
      (bind _asbp_base_bird_item (Utilities|Casting|CastToBP_BaseBirdItem _array_element))
      (Utilities|Array|Add (LocalVariables|GetnestedBirds) _asbp_base_bird_item))
    (:Completed
      (return (LocalVariables|GetnestedBirds)))))

(fn HasFreeNestingSlots
  (return (< (Class|ItemInventory|GetPopulatedItemCount (Variables|Default|GetPetInventory) 0 -1) (Variables|Default|GetmaxBirds))))

(fn PlayBirdSound
  (params (birdTemplateID :type Integer))
  (if (Networking|IsDedicatedServer)
    (return false)
    (else
      (bind _birdtype (CallFunction|GetBirdTypefromTemplateID birdTemplateID))
      (CallFunction|PlaySoundat (Variables|Default|GetBirdAudio) (Utilities|Struct|BreakSTRUCT_RACO_BirdType _birdtype))
      (return false))))

(fn UpdateBirdAnimations
  (bind _array_element (Utilities|ForEachLoopFast (Variables|Default|GetPets))
    (:LoopBody
      (Components|SkinnedMesh|SetSkinnedAssetandUpdate _array_element 0 true))
    (:Completed
      (bind (_array_element_2 _array_index) (Utilities|ForEachLoopFast (Variables|/Script/ConanSandbox.ItemInventory|GetItemList (Variables|Default|GetPetInventory)))
        (:LoopBody
          (LocalVariables|SetarrayIndex _array_index)
          (if (< (LocalVariables|GetarrayIndex) (Variables|Default|GetmaxBirds))
            (bind _asbp_base_bird_item (Utilities|Casting|CastToBP_BaseBirdItem _array_element_2)
              (:then
                (Utilities|Array|SetArrayElem (Variables|Default|GetPetSkeletalMeshes) (LocalVariables|GetarrayIndex) (.skeletalMesh (Utilities|Struct|BreakSTRUCT_RACO_BirdType (CallFunction|GetBirdTypebyID (Variables|/Game/Mods/RavencrestCouriers/Items/BP_BaseBirdItem.BP_BaseBirdItem_C|GetbirdTypeID _asbp_base_bird_item)))) true)
                (Utilities|Array|SetArrayElem (Variables|Default|GetPetIdleAnimations) (LocalVariables|GetarrayIndex) (Utilities|Array|Get(acopy) (.idleAnimations (Utilities|Struct|BreakSTRUCT_RACO_BirdType (CallFunction|GetBirdTypebyID (Variables|/Game/Mods/RavencrestCouriers/Items/BP_BaseBirdItem.BP_BaseBirdItem_C|GetbirdTypeID _asbp_base_bird_item))))) true)
                (Transformation|SetRelativeTransform (Utilities|Array|Get(acopy) (Variables|Default|GetPets) (LocalVariables|GetarrayIndex)) (select (== (Variables|/Game/Mods/RavencrestCouriers/Items/BP_BaseBirdItem.BP_BaseBirdItem_C|GetbirdTypeID _asbp_base_bird_item) "bat") (Math|Transform|ComposeTransforms (Math|Transform|ComposeTransforms (Utilities|Array|Get(acopy) (Variables|Default|GetPetOriginalTransforms)) (.transform (Utilities|Struct|BreakSTRUCT_RACO_BirdType (CallFunction|GetBirdTypebyID (Variables|/Game/Mods/RavencrestCouriers/Items/BP_BaseBirdItem.BP_BaseBirdItem_C|GetbirdTypeID _asbp_base_bird_item))))) (Variables|Default|GetbatTransform)) (Math|Transform|ComposeTransforms (Utilities|Array|Get(acopy) (Variables|Default|GetPetOriginalTransforms)) (.transform (Utilities|Struct|BreakSTRUCT_RACO_BirdType (CallFunction|GetBirdTypebyID (Variables|/Game/Mods/RavencrestCouriers/Items/BP_BaseBirdItem.BP_BaseBirdItem_C|GetbirdTypeID _asbp_base_bird_item)))))) false false))
              (:CastFailed
                (Utilities|Array|SetArrayElem (Variables|Default|GetPetSkeletalMeshes) (LocalVariables|GetarrayIndex) 0 true)
                (Utilities|Array|SetArrayElem (Variables|Default|GetPetIdleAnimations) (LocalVariables|GetarrayIndex) 0 true)
                (Transformation|SetRelativeScale3D (Utilities|Array|Get(acopy) (Variables|Default|GetPets) (LocalVariables|GetarrayIndex)) "0, 0, 0")))
            (else
              (CallFunction|SetPetVisuals :!label _label)
              (return false))))
        (:Completed
          (goto _label))))))