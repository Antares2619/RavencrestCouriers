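; BP_Coop_Medium2 is a medium coop placeable variant with twelve pet slots.
; It overrides CustomizePetSlots to gather the slot references into the Pets array and size the parallel idle animation, skeletal mesh and sound cue arrays to match.
; The construction script only calls the parent, and this file assigns no content to those resized arrays.
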(event EventCustomizePetSlots
  (bind _output_get (Variables|Default|SetPets (Utilities|Array|MakeArray (Variables|Default|GetPetSlot01) (Variables|Default|GetPetSlot02) (Variables|Default|GetPetSlot03) (Variables|Default|GetPetSlot04) (Variables|Default|GetPetSlot05) (Variables|Default|GetPetSlot06) (Variables|Default|GetPetSlot07) (Variables|Default|GetPetSlot08) (Variables|Default|GetPetSlot09) (Variables|Default|GetPetSlot10) (Variables|Default|GetPetSlot11) (Variables|Default|GetPetSlot12))))
  (Utilities|Array|Resize (Variables|Default|GetPetIdleAnimations) (Utilities|Array|Length _output_get))
  (Utilities|Array|Resize (Variables|Default|GetPetSkeletalMeshes) (Utilities|Array|Length _output_get))
  (Utilities|Array|Resize (Variables|Default|GetPetSoundCues) (Utilities|Array|Length _output_get)))

(fn ConstructionScript
  (|CallParentFunction))