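; BP_RACO_I_Nest is an interface for placeable nests that house birds.
; It declares queries for nested birds, free nesting slots and whether a given bird fits, plus a nesting action that reports success and error info.
; It also declares hooks to play a bird sound by template ID and update bird animations.
; All functions are stubs, so the file holds no nesting logic itself.
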(fn GetNestedBirds
  (return 0))

(fn HasFreeNestingSlots
  (return false))

(fn PlayBirdSound
  (params (birdTemplateID :type Integer))
  (return))

(fn UpdateBirdAnimations
  (return))

(fn NestFitsBird
  (params (bird :type Game%20Item%20Object%20Reference))
  (return false))

(fn DoNestBird
  (params (bird :type Game%20Item%20Object%20Reference))
  (return false ""))