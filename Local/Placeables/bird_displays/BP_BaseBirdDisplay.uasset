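; Base bird display placeable that shows inventory bird items as animated meshes and can act as a player proximity alarm.
; Inventory signals refresh slot mesh, anim class (async-loaded if needed) and transform relative to cached slot transforms.
; A saved config sets the active bird, radius and clan-based targets for a detection sphere, which triggers bird sound with a cooldown when server settings allow.
; Nesting functions are stubs returning false, except the population getter.
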(event SignalItemRemoved(PlaceableInventory)
  (params (index :type Integer) (item :type Game%20Item%20Object%20Reference) (dstInventory :type Item%20Inventory%20Object%20Reference) (dstIndex :type Integer))
  (RACO|RefreshBirdSlot 0 index)
  (if (Networking|IsServer)
    (RACO|Detection|RefreshDetectionConfig item dstInventory false)))

(event OnComponentBeginOverlap(DetectionSphere)
  (params (OverlappedComponent :type Primitive%20Component%20Object%20Reference) (OtherActor :type Actor%20Object%20Reference) (OtherComp :type Primitive%20Component%20Object%20Reference) (OtherBodyIndex :type Integer) (bFromSweep :type Boolean) (SweepResult :type Hit%20Result%20Structure%20%28by%20ref%29))
  (RACO|Detection|HandleDetectionEvent OtherActor))

(event SignalItemAdded(PlaceableInventory)
  (params (index :type Integer) (item :type Game%20Item%20Object%20Reference) (srcInventory :type Item%20Inventory%20Object%20Reference) (srcIndex :type Integer))
  (RACO|RefreshBirdSlot item index)
  (if (Networking|IsServer)
    (RACO|Detection|RefreshDetectionConfig item srcInventory true)))

(event Custom|asyncSetBirdSlotParameters
  (params (animClass :type AB%20Base%20Bird%20Soft%20Class%20Reference) (transform :type Transform) (birdSlot :type Skeletal%20Mesh%20Component%20Object%20Reference) (slotIndex :type Integer))
  (bind _class (Utilities|AsyncLoadClassAsset animClass)
    (:Completed
      (bind _asab_base_bird (Utilities|Casting|CastToAB_BaseBirdClass _class))
      (RACO|SetBirdSlotParameters _asab_base_bird transform birdSlot slotIndex))))

(event Custom|onTargetDetected
  (params (detectedActor :type Actor%20Object%20Reference) (activeBirdIndex :type Integer))
  (bind _placeableinventory (Variables|Default|GetPlaceableInventory))
  (bind _returnvalue (Class|ItemInventory|GetItem _placeableinventory activeBirdIndex))
  (if (not (Networking|IsDedicatedServer))
    (Utilities|IsValid _returnvalue
      (:Is%20Valid
        (bind _asbp_base_bird_item (Utilities|Casting|CastToBP_BaseBirdItem _returnvalue))
        (bind _typeid (Default|GetBirdType _asbp_base_bird_item))
        (CallFunction|PlayBirdSound (Variables|Default|GetBirdAudio) (CallFunction|GetBirdTypebyID _typeid))))))

(event EventBeginPlay
  (|CallParentFunction)
  (if (not (Variables|Default|GetIsABrush))
    (Utilities|FlowControl|Sequence
      (:then_0
        (bind _array (RACO|GetBirdSlots))
        (bind (_array_element _array_index) (Utilities|ForEachLoopFast _array)
          (:LoopBody
            (Utilities|Array|SetArrayElem (Variables|Default|GetBirdSlotsTransforms) _array_index (Transformation|GetRelativeTransform _array_element) true))))
      (:then_1
        (if (not (Networking|IsServer))
          (bind _returnvalue (Game|ConstructObjectfromClass "/Script/ConanSandbox.ItemInventoryClientMonitor"))
          (Class|ItemInventoryClientMonitor|SetInventory _returnvalue (Variables|Default|GetPlaceableInventory)))))))

(event EventCleanUp
  ;[1 1 1 0.3] Override the cleanup functionality so it does not remove Birdslots
)

(fn ConstructionScript
  (|CallParentFunction))

(fn GetBirdSlots
  (return (Utilities|Array|MakeArray (Variables|Default|GetBirdSlot01))))

(fn RefreshBirdSlot
  (params (item :type Game%20Item%20Object%20Reference) (slotIndex :type Integer))
  (bind _array (RACO|GetBirdSlots))
  (if (Utilities|Array|IsValidIndex _array slotIndex)
    (Utilities|IsValid item
      (:Is%20Valid
        (bind _asbp_base_bird_item (Utilities|Casting|CastToBP_BaseBirdItem item)
          (:then
            (bind _typeid (Default|GetBirdType _asbp_base_bird_item))
            (if (Utilities|IsValidClass (Utilities|ResolveSoftReference (.animClass (Utilities|Struct|BreakSTRUCT_RACO_BirdType (CallFunction|GetBirdTypebyID _typeid)))))
              (RACO|SetBirdSlotParameters (Utilities|ResolveSoftReference (.animClass (Utilities|Struct|BreakSTRUCT_RACO_BirdType (CallFunction|GetBirdTypebyID _typeid)))) (.transform (Utilities|Struct|BreakSTRUCT_RACO_BirdType (CallFunction|GetBirdTypebyID _typeid))) (Utilities|Array|Get(acopy) _array slotIndex) slotIndex)
              (else
                (CallFunction|AsyncSetBirdSlotParameters (.animClass (Utilities|Struct|BreakSTRUCT_RACO_BirdType (CallFunction|GetBirdTypebyID _typeid))) (.transform (Utilities|Struct|BreakSTRUCT_RACO_BirdType (CallFunction|GetBirdTypebyID _typeid))) (Utilities|Array|Get(acopy) _array slotIndex) slotIndex))))
          (:CastFailed
            (RACO|SetBirdSlotParameters :birdSlot (Utilities|Array|Get(acopy) _array slotIndex) :slotIndex slotIndex :!label _label))))
      (:Is%20Not%20Valid
        (goto _label)))))

(fn SetBirdSlotParameters
  (params (animClass :type AB%20Base%20Bird%20Class%20Reference) (transform :type Transform) (birdSlot :type Skeletal%20Mesh%20Component%20Object%20Reference) (slotIndex :type Integer))
  (bind _returnvalue (Class|DreamworldBlueprints|GetClassDefaultObject animClass))
  (bind _birdmesh (Default|GetBirdMesh _returnvalue))
  (if (Utilities|IsValidClass animClass)
    (Utilities|IsValid _birdmesh
      (:Is%20Valid
        (Components|SkinnedMesh|SetSkinnedAssetandUpdate birdSlot _birdmesh true)
        (Components|SkeletalMesh|SetAnimInstanceClass birdSlot animClass)
        (Transformation|SetRelativeTransform birdSlot (CallFunction|ApplyBirdTransform (Utilities|Array|Get(acopy) (Variables|Default|GetBirdSlotsTransforms) slotIndex) transform) false false)
        (Rendering|SetVisibility birdSlot true true))
      (:Is%20Not%20Valid
        (Rendering|SetVisibility birdSlot false true :!label _label)
        (Components|SkinnedMesh|SetSkinnedAssetandUpdate birdSlot 0 true)
        (Components|SkeletalMesh|SetAnimInstanceClass birdSlot 0)
        (Transformation|SetRelativeTransform birdSlot (Utilities|Array|Get(acopy) (Variables|Default|GetBirdSlotsTransforms) slotIndex) false false)))
    (else
      (goto _label))))

(fn RefreshAllSlots
  (bind _array (RACO|GetBirdSlots))
  (for (_ _array_index) _array
    (RACO|RefreshBirdSlot (Class|ItemInventory|GetItem (Variables|Default|GetPlaceableInventory) _array_index) _array_index)))

(fn BypassDetectionFunctionality
  (return false))

(fn SetDetectionConfig
  (params (detectionConfig :type STRUCT%20RACO%20Bird%20Detection%20Config%20Structure))
  (Variables|Default|SetdetectionConfig detectionConfig)
  (Class|PersistenceComponent|SetDirty (Variables|Default|GetConanBuildingPersistence) true 5.0))

(fn ValidateDetectionConfig
  (params (detectionConfig :type STRUCT%20RACO%20Bird%20Detection%20Config%20Structure))
  (bind (_activebirdguid _radius) (Utilities|Struct|BreakSTRUCT_RACO_BirdDetectionConfig detectionConfig))
  (bind (_activebirdguid_2 _radius_2 _targets) (Utilities|Struct|BreakSTRUCT_RACO_BirdDetectionConfig detectionConfig))
  (bind (_radius_3 _targets_2) (Utilities|Struct|BreakSTRUCT_RACO_BirdDetectionConfig detectionConfig))
  (if (Guid|IsValidGuid _activebirdguid)
    (bind (_success _bird) (RACO|Detection|GetActiveBirdbyGUID _activebirdguid))
    (if _success
      (bind _birdprofile (Default|GetBirdProfile _bird))
      (bind _detectionrange (CallFunction|CalcBirdDetectionRange _birdprofile))
      (if (<= _radius _detectionrange)
        (return true detectionConfig)
        (else
          (return false (Utilities|Struct|MakeSTRUCT_RACO_BirdDetectionConfig _activebirdguid_2 (Math|Float|Truncate _detectionrange) _targets))))
      (else
        (return false (RACO|Detection|GetDefatulDetectionConfig))))
    (else
      (return (and (== _radius_3 0) (Utilities|Enum|Equal(Enum) _targets_2 "NewEnumerator4")) (RACO|Detection|GetDefatulDetectionConfig)))))

(fn RefreshDetectionConfig
  (params (item :type Game%20Item%20Object%20Reference) (inventory :type Item%20Inventory%20Object%20Reference) (isSrcInventory :type Boolean))
  (bind _asbp_base_bird_item (Utilities|Casting|CastToBP_BaseBirdItem item))
  (bind _birdprofile (Default|GetBirdProfile _asbp_base_bird_item))
  (if (== (Utilities|Struct|BreakSTRUCT_RACO_BirdProfile _birdprofile) (Utilities|Struct|BreakSTRUCT_RACO_BirdDetectionConfig (Variables|Default|GetdetectionConfig)))
    (if (not (== (Variables|Default|GetPlaceableInventory) inventory))
      (Utilities|FlowControl|Sequence
        (:then_0
          (if (not isSrcInventory)
            (RACO|Detection|SetDetectionConfig (RACO|Detection|GetDefatulDetectionConfig))))
        (:then_1
          (RACO|Detection|ApplyDetectionConfig))))))

(fn ApplyDetectionConfig
  (bind _detectionconfig (Variables|Default|GetdetectionConfig))
  (bind (_activebirdguid _radius) (Utilities|Struct|BreakSTRUCT_RACO_BirdDetectionConfig _detectionconfig))
  (if (Guid|IsValidGuid _activebirdguid)
    (Variables|/Script/Engine.PrimitiveComponent|SetbGenerateOverlapEvents (Variables|Default|GetDetectionSphere) (Default|GetIsDetectionModeAllowed (CallFunction|GetServerSettingsRACO)))
    (Components|Sphere|SetSphereRadius (Variables|Default|GetDetectionSphere) (Math|Conversions|ToFloat(Integer) _radius) true)
    (else
      (Variables|/Script/Engine.PrimitiveComponent|SetbGenerateOverlapEvents (Variables|Default|GetDetectionSphere) false)
      (Components|Sphere|SetSphereRadius (Variables|Default|GetDetectionSphere) 32.0 true))))

(fn HandleDetectionEvent
  (params (detectedActor :type Actor%20Object%20Reference))
  (Utilities|And+Branch (Default|GetIsDetectionModeAllowed (CallFunction|GetServerSettingsRACO)) (Guid|IsValidGuid (Utilities|Struct|BreakSTRUCT_RACO_BirdDetectionConfig (Variables|Default|GetdetectionConfig)))
    (:True
      (if (>= (Math|DateTime|Now) (+ (Variables|Default|GetdetectionTime) (Math|Timespan|MakeTimespan 0 0 0 5)))
        (bind _asconan_character (Utilities|Casting|CastToConanCharacter detectedActor))
        (if (Class|ConanCharacter|IsPlayer _asconan_character)
          (switch Utilities|FlowControl|Switch|SwitchonENUM_RACO_BirdDetectionTargets (.targets (Utilities|Struct|BreakSTRUCT_RACO_BirdDetectionConfig (Variables|Default|GetdetectionConfig)))
            (:NewEnumerator0
              (if (Class|BuildableBase|IsOwner _asconan_character false)
                (CallFunction|OnTargetDetected detectedActor :!label _label)
                (Variables|Default|SetdetectionTime (Math|DateTime|Now))))
            (:NewEnumerator1
              (if (not (Class|BuildableBase|IsOwner _asconan_character false))
                (goto _label)))
            (:NewEnumerator2
              (goto _label))))))))

(fn ClientGetCraftingGUICenterPanel
  (params (Instigator :type Player%20Controller%20Object%20Reference))
  (if (RACO|Detection|BypassDetectionFunctionality)
    (bind _returnvalue (|CallParentFunction Instigator))
    (return _returnvalue)
    (else
      (return "BirdDisplayInventory"))))

(fn GetActiveBirdbyGUID
  (params (GUID :type Guid%20Structure))
  (bind _returnvalue (Class|ItemInventory|GetItemList (Variables|Default|GetPlaceableInventory)))
  (bind _array_element (Utilities|ForEachLoopFast _returnvalue)
    (:LoopBody
      (Utilities|IsValid _array_element
        (:Is%20Valid
          (bind _asbp_base_bird_item (Utilities|Casting|CastToBP_BaseBirdItem _array_element))
          (bind _birdprofile (Default|GetBirdProfile _asbp_base_bird_item))
          (if (== GUID (Utilities|Struct|BreakSTRUCT_RACO_BirdProfile _birdprofile))
            (return true _asbp_base_bird_item)))))
    (:Completed
      (return false 0))))

(fn GetDefatulDetectionConfig
  (return (Utilities|Struct|MakeSTRUCT_RACO_BirdDetectionConfig "00000000000000000000000000000000" 0 "NewEnumerator4")))

(fn GetDetectionConfig
  (return (Variables|Default|GetdetectionConfig)))

(fn GetNestPopulation
  (return (Class|ItemInventory|GetItemList (Variables|Default|GetPlaceableInventory))))

(fn HasFreeNestingSlots
  (return false))

(fn NestFitsBird
  (params (bird :type Object%20Object%20Reference))
  (return false))

(fn TryNestBird
  (params (bird :type Game%20Item%20Object%20Reference))
  (return false ""))