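; Base mailbox placeable for RACO messaging, opening a full UI for owners or when unlocked and a drop-only UI otherwise.
; A messaging endpoint component initializes either UI; the full UI toggles receiving and requests custom-name updates on close.
; Drop UI deposits are queued, then moved into the mailbox inventory.
; Off-server, unqueued items added without access return to their source, preventing double-click transfers from losing items.
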(event Custom|BindDropClientUI
  (bind _returnvalue (Class|GUIModuleController|ActivateModule (Class|GUIModuleController|GetGUIModuleController) (Utilities|Name|MakeLiteralName "RACO_Mailbox_DropGUI") true false))
  (bind _asw_mailbox_drop_gui (Utilities|Casting|CastToW_Mailbox_DropGUI _returnvalue))
  (EventDispatchers|BindEventtoSignalDepositItems _asw_mailbox_drop_gui (delegate Custom|OnSignalDepositItems)))

(event Custom|OnItemAdded
  (params (index :type Integer) (item :type Game%20Item%20Object%20Reference) (srcInventory :type Item%20Inventory%20Object%20Reference) (srcIndex :type Integer))
  (bind _returnvalue (Class|GameItem|GetOwnerInventory item))
  ;[1 1 1] Avoid items disappearing when double-clicking them in the Mailbox Drop UI
  (if (not (Math|Boolean|ORBoolean (Networking|IsServer) (>= (Utilities|Array|FindItem (Variables|Default|GetdepositQueue) item) 0) (.CanAccess (Class|PlaceableBase|CanAccessContainer (.AsPawn (Utilities|Casting|CastToPawn (Components|GetOwner srcInventory)))))))
    (if (Utilities|IsValid srcInventory)
      (Class|ItemInventory|MoveItem _returnvalue (Class|ItemInventory|GetItemIndex _returnvalue item) srcInventory srcIndex -1 false))))

(event Custom|DoDepositItems
  (params (items :type Array%20of%20Game%20Item%20Ref%20Structures))
  (for _array_element items
    (Class|ItemInventory|MoveItem (.Inventory (Utilities|Struct|BreakGameItemRef _array_element)) (.ItemIndex (Utilities|Struct|BreakGameItemRef _array_element)) (Variables|Default|GetPlaceableInventory) -1 -1 false)))

(event Custom|OnSignalDepositItems
  (params (items :type Array%20of%20Game%20Item%20Ref%20Structures))
  (Utilities|Array|Clear (Variables|Default|GetdepositQueue))
  (for _array_element items
    (bind _item (CallFunction|ResolveGameItemRef _array_element))
    (Utilities|Array|Add (Variables|Default|GetdepositQueue) _item))
  (CallFunction|DoDepositItems items))

(event Custom|OnUIClosing
  (params (window :type Window%20Root%20Object%20Reference))
  (CallFunction|UpdateBuildableName))

(event Custom|OnSignalToggleCanReceive
  (params (canReceive :type Boolean))
  (Default|DoToggleCanReceive (Variables|Default|GetBP_RACO_MessagingEndpoint_AC) canReceive))

(event Custom|BindFullClientUI
  (bind _returnvalue (Class|GUIModuleController|ActivateModule (Class|GUIModuleController|GetGUIModuleController) (Utilities|Name|MakeLiteralName "RACO_Mailbox_FullGUI") true false))
  (bind _asw_raco_mailbox_full_gui (Utilities|Casting|CastToW_RACO_Mailbox_FullGUI _returnvalue))
  (Default|InitMessagingUI _asw_raco_mailbox_full_gui (Variables|/Game/Mods/RavencrestCouriers/System/BP_RACO_MessagingEndpoint_AC.BP_RACO_MessagingEndpoint_AC_C|GetcanReceive (Variables|Default|GetBP_RACO_MessagingEndpoint_AC)))
  (EventDispatchers|BindEventtoSignalToggleCanReceive _asw_raco_mailbox_full_gui (delegate Custom|OnSignalToggleCanReceive))
  (EventDispatchers|BindEventtoSignalClosing _asw_raco_mailbox_full_gui (delegate Custom|OnUIClosing)))

(event EventBeginPlay
  (|CallParentFunction)
  (Variables|/Game/Mods/RavencrestCouriers/System/BP_RACO_MessagingEndpoint_AC.BP_RACO_MessagingEndpoint_AC_C|SetaudioComponent (Variables|Default|GetBP_RACO_MessagingEndpoint_AC) (Variables|Default|GetBirdAudio))
  ;[1 1 1] Avoid items disappearing when double-clicking them in the Mailbox Drop UI
  (EventDispatchers|BindEventtoSignalItemAdded (Variables|Default|GetPlaceableInventory) (delegate Custom|OnItemAdded)))

(event EventInteractableActivate
  (params (Component :type Primitive%20Component%20Object%20Reference) (Instigator :type Player%20Controller%20Object%20Reference) (HitIndex :type Integer) (TriggeredFromRadialWheel :type Boolean))
  (bind _returnvalue (Pawn|GetControlledPawn Instigator))
  (bind _bp_raco_messagingendpoint_ac (Variables|Default|GetBP_RACO_MessagingEndpoint_AC))
  (bind (_canaccess _containerislocked _instigatorisowner) (Class|PlaceableBase|CanAccessContainer _returnvalue))
  ;[1 1 1] Access check
  (if (or (not _containerislocked) _instigatorisowner)
    (Default|InitforMessagingUI _bp_raco_messagingendpoint_ac Instigator (Utilities|Name|MakeLiteralName "RACO_Mailbox_FullGUI") false)
    (CallFunction|BindFullClientUI)
    (else
      (Default|InitforMessagingUI _bp_raco_messagingendpoint_ac Instigator (Utilities|Name|MakeLiteralName "RACO_Mailbox_DropGUI") false)
      (CallFunction|BindDropClientUI))))

(fn ConstructionScript
  (|CallParentFunction))

(fn UpdateBuildableName
  (if (Class|BuildableBase|HasCustomBuildableName)
    (Default|ReqChangeName (Actor|GetComponentbyClass (Pawn|GetControlledPawn (Game|GetPlayerController 0)) "/Game/Mods/RavencrestCouriers/System/BP_RACO_AC.BP_RACO_AC_C") self (Class|BuildableBase|GetBuildableName false))))

(fn InteractableActivateDisabled
  (params (InteractingCharacter :type Conan%20Character%20Object%20Reference))
  (return false))

(fn ClientGetCraftingGUICenterPanel
  (params (Instigator :type Player%20Controller%20Object%20Reference))
  (bind _returnvalue (Pawn|GetControlledPawn Instigator))
  (bind (_canaccess _containerislocked _instigatorisowner) (Class|PlaceableBase|CanAccessContainer _returnvalue))
  (return (select (or (not _containerislocked) _instigatorisowner) "MailboxFullView" "MailboxDropView")))