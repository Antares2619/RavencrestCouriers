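; Base placeable for a bird that stores a profile from its placer, persists it and can act as a proximity alarm.
; Clients set the mesh by bird type and loop random idle animations, while the server waits for the settings system before configuring the detection sphere.
; Player overlaps filtered by owner/non-owner trigger the bird's sound, with a cooldown.
; A radial menu, owner-only unless overridden, routes pickup, profile and detection-config actions through the RACO component.
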(event OnComponentBeginOverlap(DetectionSphere)
  (params (OverlappedComponent :type Primitive%20Component%20Object%20Reference) (OtherActor :type Actor%20Object%20Reference) (OtherComp :type Primitive%20Component%20Object%20Reference) (OtherBodyIndex :type Integer) (bFromSweep :type Boolean) (SweepResult :type Hit%20Result%20Structure%20%28by%20ref%29))
  ;[1 1 1] Detection Mode
  (CallFunction|HandleDetectionEvent OtherActor))

(event Custom|TryInit
  (Utilities|IsValid (CallFunction|GetSettingsSystem)
    (:Is%20Valid
      (CallFunction|UpdateDetectionConfig (Variables|Default|GetbirdDetectionConfig)))
    (:Is%20Not%20Valid
      (Utilities|Time|SetTimerbyEvent (delegate Custom|TryInit) 1.0))))

(event Custom|OnPickupClicked
  (params (menuEntry :type Radial%20Menu%20Entry%20Object%20Reference))
  ;[1 1 1] Interaction
  (Default|ReqPickupBird (CallFunction|GetRACO) self))

(event Custom|OnIntruderDetected
  (params (intruder :type Actor%20Object%20Reference))
  ;[1 1 1] Detection Mode
  (CallFunction|PlayBirdSound))

(event Custom|LoopRandomBirdAnimation
  ;[1 1 1] Looping bird idle animations
  (bind _animlength (CallFunction|PlayRandomBirdAnimation (Variables|Default|GetSkeletalMesh) (Variables|Default|GetbirdTypeID)))
  (Utilities|FlowControl|Delay (+ _animlength (Math|Random|RandomFloatinRange 2.0 5.0)))
  (CallFunction|LoopRandomBirdAnimation))

(event Custom|OnViewProfileClicked
  (params (menuEntry :type Radial%20Menu%20Entry%20Object%20Reference))
  ;[1 1 1] Interaction
  (Default|ClientOpenBirdProfile2 (CallFunction|GetRACO) (Variables|Default|GetbirdProfile)))

(event Custom|OnViewDetectionConfigClicked
  (params (menuEntry :type Radial%20Menu%20Entry%20Object%20Reference))
  ;[1 1 1] Interaction
  (Default|ClientOpenBirdDetectionConfig (CallFunction|GetRACO) self))

(event EventInteractableMenu
  (params (RadialMenu :type Radial%20Menu%20Object%20Reference) (HitIndex :type Integer))
  ;[1 1 1] Interaction
  (|CallParentFunction RadialMenu HitIndex)
  (if (or (Class|BuildableBase|IsOwner (Pawn|GetControlledPawn (Widget|GetOwningPlayer RadialMenu)) false) (Variables|Default|GetDoNotRespectOwnership))
    (Utilities|FlowControl|Sequence
      (:then_0
        (bind _returnvalue (Class|RadialMenu|AddItem RadialMenu "Pick Up Bird" "Pick Up Bird" "/Game/UI/Textures/GUIs/MainRadialMenu/T_MainRadialMenuIconPickup.T_MainRadialMenuIconPickup" "None" 0))
        (EventDispatchers|BindEventtoSignalClicked _returnvalue (delegate Custom|OnPickupClicked)))
      (:then_1
        (bind _returnvalue_2 (Class|RadialMenu|AddItem RadialMenu "View Bird Profile" "View Bird Profile" "/Game/UI/Textures/GUIs/MainRadialMenu/MainRadialMenuIconStats.MainRadialMenuIconStats" "None" 0))
        (EventDispatchers|BindEventtoSignalClicked _returnvalue_2 (delegate Custom|OnViewProfileClicked)))
      (:then_2
        (bind _returnvalue_3 (Class|RadialMenu|AddItem RadialMenu "Configure Detection Mode" "Configure Detection Mode" "/Game/UI/Textures/GUIs/MainRadialMenu/Followers/T_FollowersIconBehaviourCategory.T_FollowersIconBehaviourCategory" "None" 0))
        (EventDispatchers|BindEventtoSignalClicked _returnvalue_3 (delegate Custom|OnViewDetectionConfigClicked))))))

(event EventBeginPlay
  (|CallParentFunction)
  (if (Networking|IsServer)
    (Utilities|Time|SetTimerbyEvent (delegate Custom|TryInit) 1.0)
    (else
      (CallFunction|UpdateBirdVisuals)
      (CallFunction|LoopRandomBirdAnimation))))

(event EventInteractableActivate
  (params (Component :type Primitive%20Component%20Object%20Reference) (Instigator :type Player%20Controller%20Object%20Reference) (HitIndex :type Integer) (TriggeredFromRadialWheel :type Boolean))
  (bind _returnvalue (Pawn|GetControlledPawn Instigator))
  ;[1 1 1] Interaction
  (if (or (Class|BuildableBase|IsOwner _returnvalue false) (Variables|Default|GetDoNotRespectOwnership))
    (Default|ClientOpenBirdProfile2 (Actor|GetComponentbyClass _returnvalue "/Game/Mods/RavencrestCouriers/System/BP_RACO_AC.BP_RACO_AC_C") (Variables|Default|GetbirdProfile))))

(event EventOnPlaced
  (params (PlacedBy :type Conan%20Character%20Object%20Reference))
  (Variables|Default|SetbirdProfile (Variables|/Game/Mods/RavencrestCouriers/System/BP_RACO_AC.BP_RACO_AC_C|GetbirdProfileBeingPlaced (Actor|GetComponentbyClass PlacedBy "/Game/Mods/RavencrestCouriers/System/BP_RACO_AC.BP_RACO_AC_C")))
  (Class|PersistenceComponent|SetDirty (Variables|Default|GetConanBuildingPersistence) true 5.0))

(fn ConstructionScript
  (|CallParentFunction))

(fn GetInstigatorOfPlacement
  (return (|CallParentFunction)))

(fn PlayBirdSound
  (if (not (Networking|IsDedicatedServer))
    (CallFunction|PlaySoundat (Variables|Default|GetBirdAudio) (.sound (Utilities|Struct|BreakSTRUCT_RACO_BirdType (CallFunction|GetBirdTypebyID (Utilities|Struct|BreakSTRUCT_RACO_BirdProfile (Variables|Default|GetbirdProfile))))))))

(fn UpdateDetectionConfig
  (params (config :type STRUCT%20RACO%20Bird%20Detection%20Config%20Structure))
  (bind _detectionsphere (Variables|Default|GetDetectionSphere))
  (Variables|Default|SetbirdDetectionConfig config)
  (Class|PersistenceComponent|SetDirty (Variables|Default|GetConanBuildingPersistence) true 5.0)
  (Variables|/Script/Engine.PrimitiveComponent|SetbGenerateOverlapEvents _detectionsphere (and (.detectionModeEnabled (Utilities|Struct|BreakSTRUCT_RACO_ServerSettings (Variables|/Game/Mods/RavencrestCouriers/System/BP_RACO_SettingsSystem.BP_RACO_SettingsSystem_C|GetserverSettings (CallFunction|GetSettingsSystem)))) (.detectionModeEnabled (Utilities|Struct|BreakSTRUCT_RACO_BirdDetectionConfig (Variables|Default|GetbirdDetectionConfig)))))
  (Components|Sphere|SetSphereRadius _detectionsphere (Math|Conversions|ToFloat(Integer) (.detectionRadius (Utilities|Struct|BreakSTRUCT_RACO_BirdDetectionConfig (Variables|Default|GetbirdDetectionConfig)))) true))

(fn HandleDetectionEvent
  (params (detectedActor :type Actor%20Object%20Reference))
  (bind _birddetectionconfig (Variables|Default|GetbirdDetectionConfig))
  (bind _detectiontypes (Utilities|Struct|BreakSTRUCT_RACO_BirdDetectionConfig _birddetectionconfig))
  (LocalVariables|SettheDetectedActor detectedActor)
  (if (and (.detectionModeEnabled (Utilities|Struct|BreakSTRUCT_RACO_ServerSettings (Variables|/Game/Mods/RavencrestCouriers/System/BP_RACO_SettingsSystem.BP_RACO_SettingsSystem_C|GetserverSettings (CallFunction|GetSettingsSystem)))) (Utilities|Struct|BreakSTRUCT_RACO_BirdDetectionConfig (Variables|Default|GetbirdDetectionConfig)))
    (if (>= (Math|DateTime|Now) (+ (Variables|Default|GetbirdLastDetectionTime) (Math|Timespan|MakeTimespan 0 0 0 5)))
      (bind _asbase_player_char (Utilities|Casting|CastToBasePlayerChar (LocalVariables|GettheDetectedActor)))
      (if (or (and (Class|BuildableBase|IsOwner _asbase_player_char false) (Utilities|Array|Get(acopy) _detectiontypes)) (and (not (Class|BuildableBase|IsOwner _asbase_player_char false)) (Utilities|Array|Get(acopy) _detectiontypes 1)))
        (CallFunction|OnIntruderDetected (LocalVariables|GettheDetectedActor))
        (Variables|Default|SetbirdLastDetectionTime (Math|DateTime|Now))))))

(fn UpdateBirdVisuals
  (bind _birdtypeid (Variables|Default|GetbirdTypeID))
  (bind _birdtype (CallFunction|GetBirdTypebyID _birdtypeid))
  (bind (_skeletalmesh _transform) (Utilities|Struct|BreakSTRUCT_RACO_BirdType _birdtype))
  (Transformation|SetRelativeTransform (Variables|Default|GetSkeletalMesh) _transform false false)
  (Components|SkinnedMesh|SetSkinnedAssetandUpdate (Variables|Default|GetSkeletalMesh) _skeletalmesh true))