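; Base inventory item for birds, holding a persistent bird profile and an in-transit message.
; On the dedicated server it polls for the owner inventory and its data load, then creates a missing profile or resumes a saved delivery with a startup minimum wait.
; Deliveries run on timestamp-based timers that hand the message to the owner.
; While equipped, a delay-and-gate guarded timer grants hourly passive XP, crediting partial time on unequip.
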(event Custom|onInventoryDataLoaded
  (bind _deliverymessage (Variables|Default|GetdeliveryMessage))
  (bind (_submittimestamp _travelduration _validated) (Utilities|Struct|BreakSTRUCT_RACO_MessageInFlight _deliverymessage))
  (EventDispatchers|UnbindEventfromOnSignalDataLoaded (stale EventSetData _inventory) (EventDispatchers|CreateEvent :!event Custom|onInventoryDataLoaded))
  (if (CallFunction|HasValidBirdID (Variables|Default|GetbirdProfile))
    (if _validated
      (CallFunction|ScheduleDelivery (Math|Float|Max(Float) (CallFunction|GetRemainingTime _submittimestamp _travelduration) 6e+01)))
    (else
      (CallFunction|InitNewBirdProfile (Variables|Default|GetbirdTypeID) (Variables|Default|GetbirdProfile))
      (Class|PersistenceComponent|SetDirty (Class|GameItem|GetOwnerInventory) true 5.0))))

(event Custom|onMaturedXP
  ;[1 1 1 0.3] Equip
  (Default|GiveBirdPassiveXP (CallFunction|GetExperienceSystemRACO) self 3.6e+03))

(event Custom|scheduleDelivery
  (params (timeToDelivery :type Float%20%28double-precision%29))
  ;[1 1 1 0.3] Delivery
  (if (> timeToDelivery 0.99)
    (bind _returnvalue (Utilities|Time|SetTimerbyEvent (delegate Custom|doDelivery) timeToDelivery))
    (Variables|Default|SetdeliveryTimer _returnvalue)
    (else
      (Class|BPRACOIMessagingSystem|TryDeliverMessage(Message) (Class|GameItem|GetOwner) self))))

(event Custom|doDelivery
  ;[1 1 1 0.3] Delivery
  (Class|BPRACOIMessagingSystem|TryDeliverMessage(Message) (Class|GameItem|GetOwner) self))

(event EventSetData
  (params (templateID :type Integer))
  (bind _deliverymessage (Variables|Default|GetdeliveryMessage))
  (bind (_submittimestamp _travelduration _validated) (Utilities|Struct|BreakSTRUCT_RACO_MessageInFlight _deliverymessage))
  (|CallParentFunction templateID)
  (if (Networking|IsDedicatedServer)
    (bind _inventory (Utilities|WaitforOwnerInventory)
      (:continue
        (if (CallFunction|HasValidBirdID (Variables|Default|GetbirdProfile))
          (if _validated
            (CallFunction|ScheduleDelivery (Math|Float|Max(Float) (CallFunction|GetRemainingTime _submittimestamp _travelduration) 6e+01)))
          (else
            (CallFunction|InitNewBirdProfile (Variables|Default|GetbirdTypeID) (Variables|Default|GetbirdProfile))
            (Class|PersistenceComponent|SetDirty (Class|GameItem|GetOwnerInventory) true 5.0))))
      (:dataNotLoaded
        (EventDispatchers|AssignOnSignalDataLoaded _inventory (EventDispatchers|CreateEvent :!event Custom|onInventoryDataLoaded))))))

(event EventAssignDelivery
  (params (message :type STRUCT%20RACO%20Message%20in%20Flight%20Structure))
  ;[1 1 1 0.3] Delivery
  (bind _output_get (Variables|Default|SetdeliveryMessage message))
  (CallFunction|ScheduleDelivery (CallFunction|GetRemainingTime (.submitTimestamp (Utilities|Struct|BreakSTRUCT_RACO_MessageInFlight _output_get)) (.travelDuration (Utilities|Struct|BreakSTRUCT_RACO_MessageInFlight _output_get))))
  (CallFunction|SaveItemPersistentData self))

(event EventClearDelivery
  ;[1 1 1 0.3] Delivery
  (CallFunction|ClearMessage (Variables|Default|GetdeliveryMessage))
  (Utilities|Time|ClearandInvalidateTimerbyHandle (Variables|Default|GetdeliveryTimer))
  (CallFunction|SaveItemPersistentData self))

(event EventOnEquip
  (params (owner :type Character%20Object%20Reference))
  ;[1 1 1 0.3] Equip
  (|CallParentFunction owner)
  (if (Networking|IsDedicatedServer)
    (Utilities|FlowControl|Sequence
      (:then_0
        (Utilities|FlowControl|Delay 5.0)
        (Utilities|FlowControl|Gate false :!label _label ; Ensure we haven't un-equipped this item
          (:Exit
            (bind _returnvalue (Utilities|Time|SetTimerbyEvent (delegate Custom|onMaturedXP) 3.6e+03 true))
            (Variables|Default|SetxpTimer _returnvalue))))
      (:then_1
        (goto _label Open)))))

(event EventOnUnEquip
  (params (owner :type Character%20Object%20Reference))
  ;[1 1 1 0.3] Equip
  (|CallParentFunction owner)
  (if (Networking|IsDedicatedServer)
    (Utilities|FlowControl|Sequence
      (:then_0
        (if (Utilities|Time|IsValidTimerHandle (Variables|Default|GetxpTimer))
          (Default|GiveBirdPassiveXP (CallFunction|GetExperienceSystemRACO) self (Class|KismetSystemLibrary|GetTimerElapsedTimeHandle (Variables|Default|GetxpTimer)))
          (Utilities|Time|ClearandInvalidateTimerbyHandle (Variables|Default|GetxpTimer))))
      (:then_1
        (Utilities|FlowControl|Gate false) ; enters at Close
      ))))

(fn GetStatTexts
  (bind _birdtypeid (Variables|Default|GetbirdTypeID))
  (bind _birdtype (CallFunction|GetBirdTypebyID _birdtypeid))
  (bind _size (Utilities|Struct|BreakSTRUCT_RACO_BirdType _birdtype))
  (Utilities|FlowControl|Sequence
    (:then_0
      (if (not (Utilities|Array|IsEmpty _size))
        (LocalVariables|SetlocalStatOne (Utilities|Text|ToText(String) (Utilities|String|Append (CallFunction|CapitalizeFirstLetter _size) " bird")))))
    (:then_1
      (return (LocalVariables|GetlocalStatOne) "" ""))))

(fn GetBirdProfile
  (return (Variables|Default|GetbirdProfile)))

(fn GetBirdTemplateID
  (return (Variables|Default|GetTemplateID)))

(fn GetBirdType
  (return (Variables|Default|GetbirdTypeID)))

(fn GetDetectionConfig
  (return ""))

(fn GetMessageinTransit
  (return (Variables|Default|GetdeliveryMessage)))

(fn SetBirdProfile
  (params (profile :type STRUCT%20RACO%20Bird%20Profile%20Structure))
  (Variables|Default|SetbirdProfile profile)
  (if (Networking|IsServer)
    (CallFunction|SaveItemPersistentData self)))

(fn SetDetectionConfig
  (params (newConfig :type STRUCT%20RACO%20Bird%20Detection%20Config%20Structure))
  (return false))