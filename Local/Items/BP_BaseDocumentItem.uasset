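; Base inventory item for documents, which the local player can read or place in the world.
; A short timer splits use into single tap, which opens the read view or stops active building, and double tap, which signals placement through the RACO actor component.
; Only double taps, dedicated servers and non-local users reach the parent use logic.
; Descriptions come from the Document; read and write UI module names default to None.
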(event Custom|OnSingleTap
  (Utilities|Time|ClearandInvalidateTimerbyHandle (Variables|Default|GetdelayedTimerHandle))
  (if (Variables|/Script/ConanSandbox.BuildSystemComponent|GetIsBuilding (Actor|GetComponentbyClass (stale EventOnUseItem invokingCharacter) "/Game/Systems/Building/BP_BuildSystem_v2.BP_BuildSystem_v2_C"))
    (Class|BuildSystemComponent|StopBuilding (Actor|GetComponentbyClass (stale EventOnUseItem invokingCharacter) "/Game/Systems/Building/BP_BuildSystem_v2.BP_BuildSystem_v2_C"))
    (else
      (Default|ClientOpenItemRead (Utilities|GetRACOAC) (Utilities|GetGameItemRef)))))

(event EventOnUseItem
  (params (invokingCharacter :type Conan%20Character%20Object%20Reference) (ownerPlayer :type Conan%20Character%20Object%20Reference))
  (if (Networking|IsDedicatedServer)
    (|CallParentFunction invokingCharacter ownerPlayer :!label _label)
    (elif (== invokingCharacter (Game|GetPlayerCharacter 0))
      (if (Utilities|Time|IsValidTimerHandle (Variables|Default|GetdelayedTimerHandle))
        (Utilities|Time|ClearandInvalidateTimerbyHandle (Variables|Default|GetdelayedTimerHandle))
        (Default|NotifyItemBeingPlaced (Utilities|GetRACOAC) (Utilities|GetGameItemRef))
        (goto _label)
        (else
          (bind _returnvalue (Utilities|Time|SetTimerbyEvent (delegate Custom|OnSingleTap) 0.2))
          (Variables|Default|SetdelayedTimerHandle _returnvalue)))
      (else
        (goto _label)))))

(fn GetDocReadUIModuleName
  (return "None"))

(fn GetDocWriteUIModuleName
  (return "None"))

(fn CanUseItem
  (params (invokingCharacter :type Conan%20Character%20Object%20Reference))
  (return true))

(fn CanbeActivated
  (return false))

(fn GetShortDesc
  (return (Utilities|Text|ToText(String) (CallFunction|GetDocumentDescription (Variables|Default|Getdocument) true))))

(fn GetLongDesc
  (return (Utilities|Text|ToText(String) (CallFunction|GetDocumentDescription (Variables|Default|Getdocument) false))))