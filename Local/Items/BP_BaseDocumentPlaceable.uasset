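; Base placeable actor for a readable document in the world, holding a document struct and its item template ID.
; On placement it copies both from the placer's BP_RACO_AC component and marks persistence dirty.
; Interacting opens the document GUI through that component; the radial menu adds an owner-gated Pick Up (bypassable by flag) that requests pickup there.
; UI module name getters return "None" here.
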(event Custom|OnPickupClicked
  (params (menuEntry :type Radial%20Menu%20Entry%20Object%20Reference))
  ;[1 1 1] Interaction wheel: add a custom PickUp action (that also remembers the document struct)
  (Default|ReqDocPickUp (Actor|GetComponentbyClass (Pawn|GetControlledPawn (Game|GetPlayerController 0)) "/Game/Mods/RavencrestCouriers/System/BP_RACO_AC.BP_RACO_AC_C") self))

(event EventInteractableMenu
  (params (RadialMenu :type Radial%20Menu%20Object%20Reference) (HitIndex :type Integer))
  ;[1 1 1] Interaction wheel: add a custom PickUp action (that also remembers the document struct)
  (|CallParentFunction RadialMenu HitIndex)
  (if (or (Class|BuildableBase|IsOwner (Pawn|GetControlledPawn (Widget|GetOwningPlayer RadialMenu)) false) (Variables|Default|GetDoNotRespectOwnership))
    (bind _returnvalue (Class|RadialMenu|AddItem RadialMenu "Pick Up" "Pick Up" "/Game/UI/Textures/GUIs/MainRadialMenu/T_MainRadialMenuIconPickup.T_MainRadialMenuIconPickup" "None" 0))
    (EventDispatchers|BindEventtoSignalClicked _returnvalue (delegate Custom|OnPickupClicked))))

(event EventOnPlaced
  (params (PlacedBy :type Conan%20Character%20Object%20Reference))
  (bind _returnvalue (Actor|GetComponentbyClass PlacedBy "/Game/Mods/RavencrestCouriers/System/BP_RACO_AC.BP_RACO_AC_C"))
  ;[1 1 1] After placement, retrieve document state from the RACO AC and apply to this Actor
  (Variables|Default|Setdocument (Variables|/Game/Mods/RavencrestCouriers/System/BP_RACO_AC.BP_RACO_AC_C|GetdocBeingPlaced _returnvalue))
  (Variables|Default|SetdocItemTemplateID (Variables|/Game/Mods/RavencrestCouriers/System/BP_RACO_AC.BP_RACO_AC_C|GetdocTemplateID _returnvalue))
  (Class|PersistenceComponent|SetDirty (Variables|Default|GetConanBuildingPersistence) true 5.0)
  (Default|NotifyItemPlacementDone _returnvalue))

(event EventInteractableActivate
  (params (Component :type Primitive%20Component%20Object%20Reference) (Instigator :type Player%20Controller%20Object%20Reference) (HitIndex :type Integer) (TriggeredFromRadialWheel :type Boolean))
  ;[1 1 1] Default interaction: read the document
  (bind _document (CallFunction|GetDocument))
  (Default|OpenDocumentGUIfromPlaceable (Actor|GetComponentbyClass (Pawn|GetControlledPawn Instigator) "/Game/Mods/RavencrestCouriers/System/BP_RACO_AC.BP_RACO_AC_C") self _document))

(fn ConstructionScript
  (|CallParentFunction))

(fn GetDocUIModuleName0
  (return "None"))

(fn GetDocWriteUIModuleName
  (return "None"))

(fn InteractableActivateDisabled
  (params (InteractingCharacter :type Conan%20Character%20Object%20Reference))
  (return false))

(fn GetDocItemTemplateID
  (return (Variables|Default|GetdocItemTemplateID)))

(fn GetDocUIModuleName
  (return "None"))

(fn GetDocument
  (return (Variables|Default|Getdocument)))

(fn SetDocItemTemplateID
  (params (TemplateID :type Integer))
  (Variables|Default|SetdocItemTemplateID TemplateID))

(fn SetDocument
  (params (document :type STRUCT%20RACO%20Document%20Structure))
  (Variables|Default|Setdocument document))