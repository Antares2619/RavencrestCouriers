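; BP_RACO_ModController is the mod controller for RACO, registering the mod's data and bootstrapping its systems.
; ModDataTableOperations merges RACO tables into the base UI module, crafting panel, item, recipe, feat, console command and construction subclass tables.
; On BeginPlay, the server waits briefly, then spawns each class in RACOSystems that has no existing actor, with itself as owner.
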(event EventBeginPlay
  (if (Networking|IsServer)
    (Utilities|FlowControl|Delay 3.0)
    ;[1 1 1] Spawn all required systems (Server)
    (for _array_element (Variables|Default|GetRACOSystems)
      (bind _outactors (Actor|GetAllActorsOfClass _array_element))
      (if (== (Utilities|Array|Length _outactors) 0)
        (Game|SpawnActorfromClass _array_element (Math|Conversions|ToTransform(Vector) "0, 0, 0") "Undefined" "OverrideRootScale" self 0)))))

(fn ConstructionScript)

(fn ModDataTableOperations
  (Class|ModController|MergeDataTables "/Game/UI/Data/DataTables/DT_UIModuleTable.DT_UIModuleTable" "/Game/Mods/RavencrestCouriers/DataTables/DT_RACO_UIModules.DT_RACO_UIModules")
  (Class|ModController|MergeDataTables "/Game/UI/Data/DataTables/DT_CraftingGUIPanelTable.DT_CraftingGUIPanelTable" "/Game/Mods/RavencrestCouriers/DataTables/DT_RACO_CraftingGUIPanels.DT_RACO_CraftingGUIPanels")
  (Class|ModController|MergeDataTables "/Game/Items/ItemTable.ItemTable" "/Game/Mods/RavencrestCouriers/DataTables/DT_RACO_ItemTable.DT_RACO_ItemTable")
  (Class|ModController|MergeDataTables "/Game/Items/Recipes/RecipesTable.RecipesTable" "/Game/Mods/RavencrestCouriers/DataTables/DT_RACO_Recipes.DT_RACO_Recipes")
  (Class|ModController|MergeDataTables "/Game/Items/Feats/FeatTable.FeatTable" "/Game/Mods/RavencrestCouriers/DataTables/DT_RACO_Feats.DT_RACO_Feats")
  (Class|ModController|MergeDataTables "/Game/Systems/Cheats/CustomConsoleCommandsDataTable.CustomConsoleCommandsDataTable" "/Game/Mods/RavencrestCouriers/DataTables/DT_RACO_Commands.DT_RACO_Commands")
  (Class|ModController|MergeDataTables "/Game/UI/Data/DataTables/DT_ConstructionSubClassData.DT_ConstructionSubClassData" "/Game/Mods/RavencrestCouriers/DataTables/DT_RACO_ConstructionSubClass.DT_RACO_ConstructionSubClass"))