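; Server settings actor for the RACO system, holding options for bird flight and XP, messages, image rendering, book copying, detection and tracking.
; On server BeginPlay it assigns a persistence ID if missing, registering itself for database saving.
; UpdateServerSetting switches on a setting name, converts the value, writes it into the settings struct, schedules a delayed save and prints the change.
; The settings' RepNotify handler is empty.
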(event EventBeginPlay
  (if (Networking|IsServer)
    ;[1 1 1] Register for DB persistence
    (if (not (Class|DreamworldBlueprints|IsValidID (Class|PersistenceComponent|GetUniqueID (Variables|Default|GetActorPersistence))))
      (bind _returnvalue (Class|UniqueID|GenerateUniqueID))
      (Class|DreamworldBlueprints|SetUniqueID self _returnvalue)
      (Class|PersistenceComponent|SetDirty (Variables|Default|GetActorPersistence) true 5.0))))

(fn ConstructionScript)

(fn OnRepServerSettings)

(fn UpdateServerSetting
  (params (name :type String) (value :type String))
  (LocalVariables|SetsettingName name)
  (LocalVariables|SetsettingValue value)
  (Utilities|FlowControl|Sequence
    (:then_0
      (switch string (LocalVariables|GetsettingName)
        (:Default
          (return))
        (:baseFlightDurationSec
          (Utilities|Struct|SetmembersinSTRUCT_RACO_ServerSettings (Variables|Default|GetserverSettings) (Math|Conversions|ToInteger(Byte) (LocalVariables|GetsettingValue))))
        (:checkMessageFrequencySec
          (Utilities|Struct|SetmembersinSTRUCT_RACO_ServerSettings (Variables|Default|GetserverSettings) (Math|Conversions|ToInteger(Byte) (LocalVariables|GetsettingValue))))
        (:allowRenderImages
          (Utilities|Struct|SetmembersinSTRUCT_RACO_ServerSettings (Variables|Default|GetserverSettings) (CallFunction|ToBool (LocalVariables|GetsettingValue))))
        (:birdXPPerHour
          (Utilities|Struct|SetmembersinSTRUCT_RACO_ServerSettings (Variables|Default|GetserverSettings) (Math|Conversions|ToInteger(Byte) (LocalVariables|GetsettingValue))))
        (:birdXPPerMessage
          (Utilities|Struct|SetmembersinSTRUCT_RACO_ServerSettings (Variables|Default|GetserverSettings) (Math|Conversions|ToInteger(Byte) (LocalVariables|GetsettingValue))))
        (:detectionModeEnabled
          (Utilities|Struct|SetmembersinSTRUCT_RACO_ServerSettings (Variables|Default|GetserverSettings) (CallFunction|ToBool (LocalVariables|GetsettingValue))))
        (:allowCopyBooks
          (Utilities|Struct|SetmembersinSTRUCT_RACO_ServerSettings (Variables|Default|GetserverSettings) (LocalVariables|GetsettingValue)))
        (:allowTracking
          (Utilities|Struct|SetmembersinSTRUCT_RACO_ServerSettings (Variables|Default|GetserverSettings) (CallFunction|ToBool (LocalVariables|GetsettingValue))))
        (:allowNPCTracking
          (Utilities|Struct|SetmembersinSTRUCT_RACO_ServerSettings (Variables|Default|GetserverSettings) (CallFunction|ToBool (LocalVariables|GetsettingValue))))
        (:allowPlayerTracking
          (Utilities|Struct|SetmembersinSTRUCT_RACO_ServerSettings (Variables|Default|GetserverSettings) (CallFunction|ToBool (LocalVariables|GetsettingValue))))))
    (:then_1
      (Class|PersistenceComponent|SetDirty (Variables|Default|GetActorPersistence) true 5.0)
      (Development|PrintString (Utilities|String|Append "Setting updated: " (LocalVariables|GetsettingName) " = " (LocalVariables|GetsettingValue)) true true "(R=0.000000,G=0.660000,B=1.000000,A=1.000000)" 6.0)
      (return))))