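; Bird-tracking system that finds placed birds, birds nested in coops, and characters within the range of the tracker's equipped bird profile.
; PerformTracking filters actors by distance and, for NPCs and players, server tracking settings, then builds labeled, icon-bearing items and broadcasts the updated list.
; NPC icons come from profession data tables via synchronous loads.
; Helpers give each item's distance and camera-relative HUD angle from the local player.
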(event EventBeginPlay)

(event Collision|EventActorBeginOverlap
  (params (OtherActor :type Actor%20Object%20Reference)))

(event EventTick
  (params (DeltaSeconds :type Float%20%28single-precision%29)))

(fn ConstructionScript)

(fn PerformTracking
  (params (trackerAC :type BP%20RACO%20AC%20Object%20Reference))
  (LocalVariables|Settracker (Components|GetOwner trackerAC))
  (LocalVariables|SetmaxDistance (CallFunction|CalcBirdDetectionRange (Variables|/Game/Mods/RavencrestCouriers/System/BP_RACO_AC.BP_RACO_AC_C|GetequippedBirdProfile trackerAC)))
  (Utilities|FlowControl|Sequence
    (:then_0
      (bind _outactors (Actor|GetAllActorsOfClass "/Game/Mods/RavencrestCouriers/Items/BP_BaseBirdPlaceable.BP_BaseBirdPlaceable_C"))
      (for _array_element _outactors
        (if (CallFunction|IsAllowedtoTrackActor _array_element (LocalVariables|Gettracker) (LocalVariables|GetmaxDistance))
          (bind _item (CallFunction|MakeTrackedBirdItem (Variables|/Game/Mods/RavencrestCouriers/Items/BP_BaseBirdPlaceable.BP_BaseBirdPlaceable_C|GetbirdTypeID _array_element) (Transformation|GetActorLocation _array_element)))
          (Utilities|Array|Add (LocalVariables|GettrackedItems) _item))))
    (:then_1
      (bind _outactors_2 (Actor|GetAllActorsOfClass "/Game/Mods/RavencrestCouriers/Placeables/coops/BP_BaseCoop.BP_BaseCoop_C"))
      (for _array_element_2 _outactors_2
        (if (CallFunction|IsAllowedtoTrackActor _array_element_2 (LocalVariables|Gettracker) (LocalVariables|GetmaxDistance))
          (bind _birds (Default|GetNestedBirds _array_element_2))
          (for _array_element_3 _birds
            (bind _item_2 (CallFunction|MakeTrackedBirdItem (Variables|/Game/Mods/RavencrestCouriers/Items/BP_BaseBirdItem.BP_BaseBirdItem_C|GetbirdTypeID _array_element_3) (Transformation|GetActorLocation _array_element_2)))
            (Utilities|Array|Add (LocalVariables|GettrackedItems) _item_2)))))
    (:then_2
      (bind _outactors_3 (Actor|GetAllActorsOfClass "/Game/Characters/BaseBPChar.BaseBPChar_C"))
      (for _array_element_4 _outactors_3
        (if (CallFunction|IsAllowedtoTrackActor _array_element_4 (LocalVariables|Gettracker) (LocalVariables|GetmaxDistance))
          (bind _item_3 (CallFunction|MakeTrackedCharItem _array_element_4))
          (Utilities|Array|Add (LocalVariables|GettrackedItems) _item_3))))
    (:then_3
      (Variables|Default|SetcurrentTrackedItems (LocalVariables|GettrackedItems))
      (Default|CallTrackedItemsUpdated))))

(fn GetTrackingHUDAngle
  (params (item :type STRUCT%20RACO%20Tracked%20Item%20Structure))
  (return (Math|Float|MapRangeClamped (Math|Rotator|NormalizeAxis (+ (* (.Yaw (Math|Rotator|BreakRotator (Camera|GetCameraRotation (Game|GetPlayerCameraManager 0)))) -1.0) (.Yaw (Math|Rotator|BreakRotator (Math|Rotator|FindLookatRotation (.Position (Utilities|Struct|BreakSTRUCT_RACO_TrackedItem item)) (Transformation|GetActorLocation (Game|GetPlayerCharacter 0))))))) -1.8e+02 1.8e+02 0.0 3.6e+02)))

(fn GetTrackedItemDistance
  (params (item :type STRUCT%20RACO%20Tracked%20Item%20Structure))
  (return (Math|Vector|VectorLength (- (Utilities|Struct|BreakSTRUCT_RACO_TrackedItem item) (Transformation|GetActorLocation (Game|GetPlayerCharacter 0))))))

(fn MakeTrackedBirdItem
  (params (birdTypeID :type Name) (location :type Vector))
  (bind _birdtype (CallFunction|GetBirdTypebyID birdTypeID))
  (bind (_name _icon) (Utilities|Struct|BreakSTRUCT_RACO_BirdType _birdtype))
  (bind _returnvalue (Class|FuncomGenericLibrary|SyncLoadAsset _icon))
  (return (Utilities|Struct|MakeSTRUCT_RACO_TrackedItem _name (.AsTexture%202D (Utilities|Casting|CastToTexture2D _returnvalue)) location)))

(fn MakeTrackedCharItem
  (params (char :type Base%20BP%20Char%20Object%20Reference))
  (LocalVariables|SetcharToTrack char)
  (Utilities|FlowControl|Sequence
    (:then_0
      (bind _asbase_npc (Utilities|Casting|CastToBaseNPC (LocalVariables|GetcharToTrack))
        (:then
          (bind _returnvalue (Utilities|GetDataTableRow "/Game/Systems/SpawnTable/SpawnDataTable.SpawnDataTable" (Variables|/Script/ConanSandbox.ConanCharacter|GetSourceSpawnTable _asbase_npc))
            (:then
              (if (Utilities|Name|NotEqual(Name) (.ProfessionTemplate (Utilities|Struct|BreakSpawnTableRow _returnvalue)) "Default")
                (bind _returnvalue_2 (Utilities|GetDataTableRow "/Game/Systems/SpawnTable/ProfessionTemplateDataTable.ProfessionTemplateDataTable" (.ProfessionTemplate (Utilities|Struct|BreakSpawnTableRow _returnvalue)))
                  (:then
                    (bind _returnvalue_3 (Class|FuncomGenericLibrary|SyncLoadAsset (.Icon (Utilities|Struct|BreakProfessionTemplateTableRow _returnvalue_2))))
                    (bind _astexture_2d (Utilities|Casting|CastToTexture2D _returnvalue_3))
                    (LocalVariables|SeticonToUse _astexture_2d)))))))
        (:CastFailed
          (if (Class|GameplayStatics|ObjectIsA (LocalVariables|GetcharToTrack) "/Game/Characters/BasePlayerChar.BasePlayerChar_C")
            (LocalVariables|SeticonToUse "/Game/UI/Textures/Icons/Items/icon_charcustom_headhairstyle.icon_charcustom_headhairstyle")))))
    (:then_1
      (return (Utilities|Struct|MakeSTRUCT_RACO_TrackedItem (Class|ConanCharacter|GetCharacterName (LocalVariables|GetcharToTrack)) (LocalVariables|GeticonToUse) (Transformation|GetActorLocation (LocalVariables|GetcharToTrack)))))))

(fn IsAllowedtoTrackActor
  (params (actor :type Actor%20Object%20Reference) (tracker :type Actor%20Object%20Reference) (maxDistance :type Float%20%28double-precision%29))
  (bind _settings (CallFunction|GetServerSettings))
  (bind _settings_2 (CallFunction|GetServerSettings))
  (bind (_allowtracking _allowplayertracking) (Utilities|Struct|BreakSTRUCT_RACO_ServerSettings _settings))
  (bind (_allowtracking_2 _allownpctracking) (Utilities|Struct|BreakSTRUCT_RACO_ServerSettings _settings_2))
  (LocalVariables|SettargetActor actor)
  (LocalVariables|SettrackerActor tracker)
  (Utilities|FlowControl|Sequence
    (:then_0
      (Utilities|Casting|CastToBaseNPC (LocalVariables|GettargetActor))
      (Utilities|And+Branch _allowtracking_2 _allownpctracking
        (:False
          (return false))))
    (:then_1
      (Utilities|Casting|CastToBasePlayerChar (LocalVariables|GettargetActor))
      (Utilities|And+Branch _allowtracking _allowplayertracking
        (:False
          (return false))))
    (:then_2
      (return (and (<= (Transformation|GetDistanceTo (LocalVariables|GettargetActor) (LocalVariables|GettrackerActor)) maxDistance) (!= (LocalVariables|GettargetActor) (LocalVariables|GettrackerActor)))))))