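; Persistent messaging hub for RACO bird mail in Conan, carrying items between registered messaging endpoints.
; TrySendMessage validates the request, moves bird and payload into a transit inventory, and queues a message timed by bird speed and load weight.
; A timer, started once server settings load, delivers elapsed messages to endpoints resolved by persistent UID, awarding bird XP.
; Missing recipients send messages back to the sender; if both are missing, items are destroyed.
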(event Custom|ProcessMessageQueueEvent
  ;[1 1 1] Start processing the message queue every X seconds
  (CallFunction|ProcessMessageQueue))

(event Custom|TryInit
  ;[1 1 1] Wait until SettingsSystem is available
  (Utilities|IsValid+Branch (CallFunction|GetSettingsSystem) true
    (:True
      ;[1 1 1] Start processing the message queue every X seconds
      (Utilities|Time|SetTimerbyEvent (delegate Custom|ProcessMessageQueueEvent) (Math|Conversions|ToFloat(Integer) (.checkMessageFrequencySec (Utilities|Struct|BreakSTRUCT_RACO_ServerSettings (CallFunction|GetServerSettings)))) true))
    (:False%20or%20Invalid
      (Utilities|Time|SetTimerbyEvent (delegate Custom|TryInit) 1.0))))

(event EventBeginPlay
  (Utilities|FlowControl|Sequence
    (:then_0
      ;[1 1 1] Register for DB persistence
      (if (not (Class|DreamworldBlueprints|IsValidID (Class|PersistenceComponent|GetUniqueID (Variables|Default|GetConanBuildingPersistence))))
        (bind _returnvalue (Class|UniqueID|GenerateUniqueID))
        (Class|DreamworldBlueprints|SetUniqueID self _returnvalue)
        (Class|PersistenceComponent|SetDirty (Variables|Default|GetConanBuildingPersistence) true 5.0)))
    (:then_1
      ;[1 1 1] Wait until SettingsSystem is available
      (Utilities|Time|SetTimerbyEvent (delegate Custom|TryInit) 1.0))))

(fn ConstructionScript)

(fn TrySendMessage
  (params (senderID :type String) (receiverID :type String) (carrier :type Game%20Item%20Ref%20Structure) (payload :type Array%20of%20Game%20Item%20Ref%20Structures))
  (LocalVariables|Setsender senderID)
  (LocalVariables|Setreceiver receiverID)
  (LocalVariables|SetcarrierRef carrier)
  (LocalVariables|SetpayloadRefs payload)
  (bind _item (CallFunction|ResolveGameItemRef (LocalVariables|GetcarrierRef)))
  (LocalVariables|Setbird (.AsBP%20Base%20Bird%20Item (Utilities|Casting|CastToBP_BaseBirdItem _item)))
  (LocalVariables|SetweightPct (/ (CallFunction|GetTotalItemsWeight (LocalVariables|GetpayloadRefs)) (CallFunction|CalcBirdCarryWeight (Variables|/Game/Mods/RavencrestCouriers/Items/BP_BaseBirdItem.BP_BaseBirdItem_C|GetbirdProfile (LocalVariables|Getbird)))))
  (Utilities|FlowControl|Sequence
    (:then_0
      ;[1 1 1] Message Validation
      (Utilities|FlowControl|Sequence
        (:then_0
          (if (not (Class|DreamworldBlueprints|IsValidID (Class|UniqueID|MakeUID (LocalVariables|Getsender))))
            (return false "Invalid sender ID" "")))
        (:then_1
          (if (not (Class|DreamworldBlueprints|IsValidID (Class|UniqueID|MakeUID (LocalVariables|Getreceiver))))
            (return false "Invalid recipient ID" "")))
        (:then_2
          (if (not (Utilities|IsValid (LocalVariables|Getbird)))
            (return false "Invalid bird" "")))
        (:then_3
          (if (== (Class|GameItem|GetOwnerInventory (LocalVariables|Getbird)) (Variables|Default|GetTransitItemInventory))
            (return false "This bird is currently in transit and unavailable" "")))
        (:then_4
          (if (Utilities|Array|IsEmpty (LocalVariables|GetpayloadRefs))
            (return false "No payload in message" "")))
        (:then_5
          (bind _hasfree (CallFunction|TransitHasSlotsFree (+ (Utilities|Array|Length (LocalVariables|GetpayloadRefs)) 1)))
          (if (not _hasfree)
            (return false "Message system congested, please try again later" "")))
        (:then_6
          (if (> (LocalVariables|GetweightPct) 1.0)
            (return false "The items are too heavy for this bird to carry" "")))))
    (:then_1
      ;[1 1 1] Move payload into transit
      (bind _transitslot (CallFunction|AddItemtoTransit (LocalVariables|GetcarrierRef)))
      (Utilities|Array|Add (LocalVariables|GettransitSlots) _transitslot)
      (for _array_element (LocalVariables|GetpayloadRefs)
        (bind _transitslot_2 (CallFunction|AddItemtoTransit _array_element))
        (Utilities|Array|Add (LocalVariables|GettransitSlots) _transitslot_2)))
    (:then_2
      ;[1 1 1] Prepare a MessageRequest struct
      (bind _structout (Utilities|Struct|SetmembersinSTRUCT_RACO_MessageInFlight (LocalVariables|GetmessageReq) (Math|DateTime|Now) (LocalVariables|Getsender) (LocalVariables|Getreceiver) (Variables|/Script/ConanSandbox.GameItem|GetTemplateID (LocalVariables|Getbird)) (LocalVariables|GettransitSlots)))
      (bind _travelduration (CallFunction|CalculateTravelDuration _structout (Variables|/Game/Mods/RavencrestCouriers/Items/BP_BaseBirdItem.BP_BaseBirdItem_C|GetbirdProfile (LocalVariables|Getbird)) (LocalVariables|GetweightPct)))
      (bind _structout_2 (Utilities|Struct|SetmembersinSTRUCT_RACO_MessageInFlight _structout _travelduration))
      (LocalVariables|SetmessageReq _structout_2))
    (:then_3
      ;[1 1 1] Register the message in the queue
      (Utilities|Array|Add (Variables|Default|GetmessagesInFlight) (LocalVariables|GetmessageReq))
      (Class|PersistenceComponent|SetDirty (Variables|Default|GetConanBuildingPersistence) true 5.0))
    (:then_4
      (return true "" (LocalVariables|GetmessageReq)))))

(fn RegisterEndpoint
  (params (endpoint :type BP%20RACO%20Messaging%20Endpoint%20AC%20Object%20Reference))
  (Utilities|Array|AddUnique (Variables|Default|Getendpoints) endpoint))

(fn UnregisterEndpoint
  (params (endpoint :type BP%20RACO%20Messaging%20Endpoint%20AC%20Object%20Reference))
  (Utilities|Array|RemoveItem (Variables|Default|Getendpoints) endpoint))

(fn GetAvailableDestinations
  (params (sender :type BP%20RACO%20Messaging%20Endpoint%20AC%20Object%20Reference))
  (bind _output_get (LocalVariables|SetlocalEndpoints (Variables|Default|Getendpoints)))
  (Utilities|Array|RemoveItem _output_get sender)
  (Default|SerializetoArray (LocalVariables|GetlocalEndpoints) (LocalVariables|GetseralizedDestinations) true)
  (return (LocalVariables|GetseralizedDestinations)))

(fn ProcessMessageQueue
  (if (Utilities|Array|IsNotEmpty (Variables|Default|GetmessagesInFlight))
    (bind (_arrayindex _arrayelement) (Utilities|Array|ReverseforEachLoop (Variables|Default|GetmessagesInFlight))
      (:LoopBody
        (if (CallFunction|HasTimePassed (.submitTimestamp (Utilities|Struct|BreakSTRUCT_RACO_MessageInFlight _arrayelement)) (.travelDuration (Utilities|Struct|BreakSTRUCT_RACO_MessageInFlight _arrayelement)))
          (CallFunction|DeliverMessageNow _arrayelement)
          (Utilities|Array|RemoveIndex (Variables|Default|GetmessagesInFlight) _arrayindex)
          (Class|PersistenceComponent|SetDirty (Variables|Default|GetConanBuildingPersistence) true 5.0))))))

(fn DeliverMessageNow
  (params (message :type STRUCT%20RACO%20Message%20in%20Flight%20Structure))
  (bind _output_get (LocalVariables|SetlocalMessage message))
  (bind _endpoint (CallFunction|GetEndpointbyUID (.senderID (Utilities|Struct|BreakSTRUCT_RACO_MessageInFlight _output_get))))
  (LocalVariables|Setsender _endpoint)
  (bind _endpoint_2 (CallFunction|GetEndpointbyUID (.recipientID (Utilities|Struct|BreakSTRUCT_RACO_MessageInFlight _output_get))))
  (LocalVariables|Setreceiver _endpoint_2)
  (Utilities|FlowControl|Sequence
    (:then_0
      (bind _asbp_base_bird_item (Utilities|Casting|CastToBP_BaseBirdItem (Class|ItemInventory|GetItem (Variables|Default|GetTransitItemInventory) (Utilities|Array|Get(acopy) (Utilities|Struct|BreakSTRUCT_RACO_MessageInFlight (LocalVariables|GetlocalMessage))))))
      (Default|GiveBirdMessagingXP (CallFunction|GetExperienceSystem) _asbp_base_bird_item))
    (:then_1
      (Utilities|IsValid (LocalVariables|Getreceiver)
        (:Is%20Valid
          (Default|DoReceiveMessage (LocalVariables|Getreceiver) (LocalVariables|GetlocalMessage) :!label _label)
          (Default|HandleMessageDeliveredNotification (LocalVariables|Getsender) (LocalVariables|GetlocalMessage)))
        (:Is%20Not%20Valid
          ;[1 1 1] Return to sender
          (Utilities|IsValid (LocalVariables|Getsender)
            (:Is%20Valid
              (LocalVariables|Setreceiver (LocalVariables|Getsender))
              (goto _label))
            (:Is%20Not%20Valid
              (CallFunction|DestroyMessage (LocalVariables|GetlocalMessage)))))))))

(fn CalculateTravelDuration
  (params (message :type STRUCT%20RACO%20Message%20in%20Flight%20Structure) (carrierProfile :type STRUCT%20RACO%20Bird%20Profile%20Structure) (weightPct :type Float%20%28double-precision%29))
  (if (<= weightPct 0.5)
    _
    (elif (<= weightPct 0.75)
      (LocalVariables|SetweightFactor 1.5)
      (else
        (LocalVariables|SetweightFactor 2.0))))
  (return (Math|Float|Truncate (* (/ (Math|Conversions|ToFloat(Integer) (.baseFlightDurationSec (Utilities|Struct|BreakSTRUCT_RACO_ServerSettings (CallFunction|GetServerSettings)))) (CallFunction|CalcBirdTravelSpeed carrierProfile)) (LocalVariables|GetweightFactor)))))

(fn AddItemtoTransit
  (params (itemRef :type Game%20Item%20Ref%20Structure))
  (bind (_inventory _itemindex) (Utilities|Struct|BreakGameItemRef itemRef))
  (bind _output_get (LocalVariables|SetfreeSlotIndex (Class|ItemInventory|GetFirstFreeIndex (Variables|Default|GetTransitItemInventory) false)))
  (if (>= _output_get 0)
    (bind _returnvalue (Class|ItemInventory|MoveItem _inventory _itemindex (Variables|Default|GetTransitItemInventory) (LocalVariables|GetfreeSlotIndex) -1 false))
    (if _returnvalue
      (return (LocalVariables|GetfreeSlotIndex))
      (else
        (return -1)))
    (else
      (return -1))))

(fn GetItemfromTransit
  (params (transitSlot :type Integer) (targetInventory :type Item%20Inventory%20Object%20Reference))
  (if (>= transitSlot 0)
    (bind _returnvalue (Class|ItemInventory|MoveItem (Variables|Default|GetTransitItemInventory) transitSlot targetInventory -1 -1 true))
    (return _returnvalue)
    (else
      (return false))))

(fn TransitHasSlotsFree
  (params (freeSlotCount :type Integer))
  (bind _transititeminventory (Variables|Default|GetTransitItemInventory))
  (return (<= freeSlotCount (- (Variables|/Script/ConanSandbox.ItemInventory|GetMaxItemCount _transititeminventory) (Class|ItemInventory|GetPopulatedItemCount _transititeminventory 0 -1)))))

(fn GetEndpointbyUID
  (params (uniqueID :type String))
  (bind _actor (Class|BaseGameModeInterface|GetActorbyUniqueIDInterface(Message) (Game|GetGameMode) (Class|UniqueID|MakeUID uniqueID)))
  (return (Actor|GetComponentbyClass _actor "/Game/Mods/RavencrestCouriers/System/BP_RACO_MessagingEndpoint_AC.BP_RACO_MessagingEndpoint_AC_C")))

(fn DestroyMessage
  (params (message :type STRUCT%20RACO%20Message%20in%20Flight%20Structure))
  (bind _array_element (Utilities|ForEachLoopFast (Utilities|Struct|BreakSTRUCT_RACO_MessageInFlight message))
    (:LoopBody
      (Class|ItemInventory|DeleteItems (Variables|Default|GetTransitItemInventory) _array_element "messageLost" -1))))