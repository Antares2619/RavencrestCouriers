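; BP_RACO_ExperienceSystem awards experience and levels to RACO birds, both passively and for messaging.
; Once the settings system is available, polled every second, an hourly timer grants server-configured XP to each player character's equipped shoulder bird.
; Passive and messaging awards share GiveBirdXP, which updates the bird profile and adds an unspent point per level gained.
; Levels derive from the "Normal" curve rows in the NPC level curve data table.
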(event Custom|TryInit
  ;[1 1 1] Wait until SettingsSystem is available
  (Utilities|IsValid+Branch (CallFunction|GetSettingsSystem) true
    (:True
      ;[1 1 1] Give shoulder birds passive XP every hour
      (Utilities|Time|SetTimerbyEvent (delegate Custom|DistributePassiveXP) 3.6e+03 true))
    (:False%20or%20Invalid
      (Utilities|Time|SetTimerbyEvent (delegate Custom|TryInit) 1.0))))

(event Custom|DistributePassiveXP
  ;[1 1 1] Give shoulder birds passive XP every hour
  (bind _outactors (Actor|GetAllActorsOfClass "/Game/Characters/BasePlayerChar.BasePlayerChar_C"))
  (for _array_element _outactors
    (if (Utilities|IsValid (Variables|/Game/Mods/RavencrestCouriers/System/BP_RACO_AC.BP_RACO_AC_C|GetequippedBird (Actor|GetComponentbyClass _array_element "/Game/Mods/RavencrestCouriers/System/BP_RACO_AC.BP_RACO_AC_C")))
      (CallFunction|GiveBirdPassiveXP (Variables|/Game/Mods/RavencrestCouriers/System/BP_RACO_AC.BP_RACO_AC_C|GetequippedBird (Actor|GetComponentbyClass _array_element "/Game/Mods/RavencrestCouriers/System/BP_RACO_AC.BP_RACO_AC_C"))))))

(event EventBeginPlay
  ;[1 1 1] Wait until SettingsSystem is available
  (Utilities|Time|SetTimerbyEvent (delegate Custom|TryInit) 1.0))

(fn ConstructionScript)

(fn GiveBirdPassiveXP
  (params (bird :type BP%20Base%20Bird%20Item%20Object%20Reference))
  (CallFunction|GiveBirdXP bird (.birdXPPerHour (Utilities|Struct|BreakSTRUCT_RACO_ServerSettings (CallFunction|GetServerSettings)))))

(fn GiveBirdMessagingXP
  (params (bird :type BP%20Base%20Bird%20Item%20Object%20Reference))
  (CallFunction|GiveBirdXP bird (.birdXPPerMessage (Utilities|Struct|BreakSTRUCT_RACO_ServerSettings (CallFunction|GetServerSettings)))))

(fn GiveBirdXP
  (params (bird :type BP%20Base%20Bird%20Item%20Object%20Reference) (amount :type Integer))
  (LocalVariables|SetbirdItem bird)
  (LocalVariables|SetbirdProfile (Variables|/Game/Mods/RavencrestCouriers/Items/BP_BaseBirdItem.BP_BaseBirdItem_C|GetbirdProfile bird))
  (LocalVariables|SetxpAmount amount)
  (Utilities|FlowControl|Sequence
    (:then_0
      ;[1 1 1] Increase Experience Points
      (bind _structout (Utilities|Struct|SetmembersinSTRUCT_RACO_BirdProfile (LocalVariables|GetbirdProfile) (+ (LocalVariables|GetxpAmount) (Utilities|Struct|BreakSTRUCT_RACO_BirdProfile (LocalVariables|GetbirdProfile)))))
      (LocalVariables|SetbirdProfile _structout))
    (:then_1
      ;[1 1 1] Increase Level if applicable
      (bind _output_get (LocalVariables|SetnewLevel (CallFunction|CalculateLevel (.experience (Utilities|Struct|BreakSTRUCT_RACO_BirdProfile (LocalVariables|GetbirdProfile))))))
      (if (> _output_get (.level (Utilities|Struct|BreakSTRUCT_RACO_BirdProfile (LocalVariables|GetbirdProfile))))
        (bind _structout_2 (Utilities|Struct|SetmembersinSTRUCT_RACO_BirdProfile (LocalVariables|GetbirdProfile) (LocalVariables|GetnewLevel) (+ (- (LocalVariables|GetnewLevel) (.level (Utilities|Struct|BreakSTRUCT_RACO_BirdProfile (LocalVariables|GetbirdProfile)))) (.unspentPoints (Utilities|Struct|BreakSTRUCT_RACO_BirdProfile (LocalVariables|GetbirdProfile))))))
        (LocalVariables|SetbirdProfile _structout_2)))
    (:then_2
      (Variables|/Game/Mods/RavencrestCouriers/Items/BP_BaseBirdItem.BP_BaseBirdItem_C|SetbirdProfile (LocalVariables|GetbirdItem) (LocalVariables|GetbirdProfile)))))

(fn CalculateLevel
  (params (xp :type Integer))
  (LocalVariables|Setexperience xp)
  (bind _outrownames (DataTable|GetDataTableRowNames "/Game/Systems/Thrall/NPCLevelCurveDataTable.NPCLevelCurveDataTable"))
  (for _array_element _outrownames
    (bind _returnvalue (Utilities|GetDataTableRow "/Game/Systems/Thrall/NPCLevelCurveDataTable.NPCLevelCurveDataTable" _array_element)
      (:then
        (if (and (Utilities|Name|Equal(Name) (.CurveName (Utilities|Struct|BreakNPCProgressionCurveRow _returnvalue)) "Normal") (>= (LocalVariables|Getexperience) (.XPRequired (Utilities|Struct|BreakNPCProgressionCurveRow _returnvalue))))
          (LocalVariables|SetmatchingLevel (+ (.Level (Utilities|Struct|BreakNPCProgressionCurveRow _returnvalue)) 1))))))
  (return (LocalVariables|GetmatchingLevel)))