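; Actor component that makes a buildable a sending and receiving endpoint for bird-carried item messages.
; On the server it polls for the messaging system, registers with it and submits outgoing messages through it.
; Received payloads move from transit to the owner's inventory, minus the bird, which returns to the sender on delivery if that owner has a nest.
; It also supplies destinations to the UI, persists a can-receive toggle and plays bird sounds.
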(event Custom|TrySendMessage
  (params (carrier :type Game%20Item%20Ref%20Structure) (items :type Array%20of%20Game%20Item%20Ref%20Structures) (recipientID :type String))
  ;[1 1 1] Try to submit a message
  (bind (_accepted _errormessage _message) (Default|TrySendMessage (Utilities|GetMessagingSystem) (CallFunction|GetUniqueID) recipientID carrier items))
  (CallFunction|TriggerSignalMessageSent _accepted _errormessage _message))

(event Custom|handleMessageDeliveredNotification
  (params (message :type STRUCT%20RACO%20Message%20in%20Flight%20Structure))
  (bind (_birdtemplateid _itemtransitslots) (Utilities|Struct|BreakSTRUCT_RACO_MessageInFlight message))
  (bind _returnvalue (Components|GetOwner))
  ;[1 1 1] A message sent from this endpoint has reached its destination
  (CallFunction|TriggerSignalMessageDelivered _birdtemplateid)
  (if (CallFunction|HasNest _returnvalue)
    (bind _hasfreeslots (Class|BPRACOINest|HasFreeNestingSlots(Message) _returnvalue))
    (Default|GetItemfromTransit (Utilities|GetMessagingSystem) (Utilities|Array|Get(acopy) _itemtransitslots) (Utilities|GetOwnerInventory (select _hasfreeslots "PetInventory" "PlaceableInventory")))))

(event Custom|DoReceiveMessage
  (params (message :type STRUCT%20RACO%20Message%20in%20Flight%20Structure))
  (bind (_birdtemplateid _itemtransitslots) (Utilities|Struct|BreakSTRUCT_RACO_MessageInFlight message))
  ;[1 1 1] Receive a message
  (bind (_array_element _array_index) (Utilities|ForEachLoopFast _itemtransitslots)
    (:LoopBody
      ;;[1 1 1] Skip first item: the bird
      (if (> _array_index 0)
        (Default|GetItemfromTransit (Utilities|GetMessagingSystem) _array_element (Utilities|GetOwnerInventory "PlaceableInventory"))))
    (:Completed
      (CallFunction|TriggerSignalMessageReceived _birdtemplateid))))

(event Custom|TriggerSignalMessageReceived
  (params (carrierID :type Integer))
  ;[1 1 1] Receive a message
  (CallFunction|PlayBirdSound carrierID))

(event Custom|TriggerSignalMessageSent
  (params (accepted :type Boolean) (errorMessage :type String) (messageRequest :type STRUCT%20RACO%20Message%20in%20Flight%20Structure))
  ;[1 1 1] Try to submit a message
  (Default|CallSignalMessageSent accepted errorMessage messageRequest)
  (if accepted
    (CallFunction|PlayBirdSound (Utilities|Struct|BreakSTRUCT_RACO_MessageInFlight messageRequest))))

(event Custom|TryInit
  ;[1 1 1] Wait until MessagingSystem is available
  (Utilities|IsValid (Utilities|GetMessagingSystem)
    (:Is%20Valid
      ;[1 1 1] Register/unregister this messaging endpoint in the messaging system
      (Default|RegisterEndpoint (Utilities|GetMessagingSystem) self))
    (:Is%20Not%20Valid
      (Utilities|Time|SetTimerbyEvent (delegate Custom|TryInit) 1.0))))

(event Custom|DoToggleCanReceive
  (params (canReceive :type Boolean))
  ;[1 1 1] Toggle the "Can Receive" state
  (Variables|Default|SetcanReceive canReceive)
  (Class|PersistenceComponent|SetDirty (Actor|GetComponentbyClass (Components|GetOwner) "/Script/ConanSandbox.ConanBuildingPersistenceComponent") true 5.0))

(event Custom|TriggerSignalMessageDelivered
  (params (birdTemplateID :type Integer))
  ;[1 1 1] A message sent from this endpoint has reached its destination
  (CallFunction|PlayBirdSound birdTemplateID))

(event EventEndPlay
  (params (EndPlayReason :type EEndPlayReason%20Enum :default "Destroyed"))
  ;[1 1 1] Register/unregister this messaging endpoint in the messaging system
  (if (Networking|IsServer)
    (if (not (CallFunction|IsABrush (Components|GetOwner)))
      (Default|UnregisterEndpoint (Utilities|GetMessagingSystem) self))))

(event EventBeginPlay
  (if (Networking|IsServer)
    (if (not (CallFunction|IsABrush (Components|GetOwner)))
      ;[1 1 1] Wait until MessagingSystem is available
      (Utilities|Time|SetTimerbyEvent (delegate Custom|TryInit) 1.0))))

(fn InitforMessagingUI
  (params (instigator :type Player%20Controller%20Object%20Reference) (guiModuleName :type Name) (getDestinations :type Boolean))
  (bind _returnvalue (Components|GetOwner))
  (bind _returnvalue_2 (Pawn|GetControlledPawn instigator))
  (bind _asconan_character (Utilities|Casting|CastToConanCharacter _returnvalue_2))
  (Utilities|FlowControl|Sequence
    (:then_0
      (Actor|SetOwner _returnvalue _asconan_character)
      (Class|ConanCharacter|SetInteractingActor _asconan_character _returnvalue guiModuleName))
    (:then_1
      (if getDestinations
        (bind _destinations (Default|GetAvailableDestinations (Utilities|GetMessagingSystem) self))
        (return _destinations)
        (else
          (return (Utilities|Array|MakeArray)))))))

(fn GetDisplayName
  (bind _returnvalue (Components|GetOwner))
  (bind _asbuildable_base (Utilities|Casting|CastToBuildableBase _returnvalue))
  (bind _returnvalue_2 (Class|BuildableBase|GetOwnerName _asbuildable_base))
  (return (Utilities|String|Append (Utilities|String|ToString(Text) _returnvalue_2) " (" (Utilities|String|ToString(Text) (Class|BuildableBase|GetBuildableName _asbuildable_base false)) ")")))

(fn PlayBirdSound
  (params (birdTemplateID :type Integer))
  (if (not (Networking|IsDedicatedServer))
    (Utilities|IsValid (Variables|Default|GetaudioComponent)
      (:Is%20Valid
        (Utilities|FlowControl|Sequence
          (:then_0
            (bind _birdtype (CallFunction|GetBirdTypefromTemplateID birdTemplateID))
            (if false
              (LocalVariables|SetsoundtoPlay (.sound (Utilities|Struct|BreakSTRUCT_RACO_BirdType _birdtype)))))
          (:then_1
            (bind _returnvalue (Class|FuncomGenericLibrary|SyncLoadAsset (LocalVariables|GetsoundtoPlay)))
            (Class|ConanAudioComponent|SetSound (Variables|Default|GetaudioComponent) (.AsSound%20Base (Utilities|Casting|CastToSoundBase _returnvalue))))
          (:then_2
            (bind _outactors (Actor|GetAllActorsOfClass "/Game/Systems/BP_ServerSettings.BP_ServerSettings_C"))
            (Variables|/Script/ConanSandbox.ConanAudioComponent|SetAttenuationOverrides (Variables|Default|GetaudioComponent) (Utilities|Struct|MakeSoundAttenuationSettings (Math|Float|Max(Float) (Variables|/Script/ConanSandbox.ServerSettings|GetChatLocalRadius (Utilities|Array|Get(acopy) _outactors)) 5e+02)))
            (Class|ConanAudioComponent|Play (Variables|Default|GetaudioComponent) 0.0)))))))

(fn SerializetoArray
  (params (Array :type Array%20of%20Strings) (destinationsOnly :type Boolean%20%28by%20ref%29))
  (Utilities|Or+Branch (not destinationsOnly) (Variables|Default|GetcanReceive)
    (:True
      (bind _name (CallFunction|GetDisplayName))
      (Utilities|Array|Add Array (Utilities|String|Append _name "#" (CallFunction|GetUniqueID))))))

(fn GetUniqueID
  (return (Class|DreamworldBlueprints|ToString(UniqueID) (Class|UniqueID|GetActorUID (Components|GetOwner)))))