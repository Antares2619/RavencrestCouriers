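; RACO character component for Conan Exiles that runs player-side logic for readable documents and companion birds.
; Client events open GUI modules, while req events edit item data and return it through callback dispatchers.
; Documents support writing, seal breaking, copying and inventory syncing; birds support profiles, placement, equipping and timed tracking.
; OnRep attaches the equipped bird's animated mesh to the shoulder, and a spawned off-world room provides profile previews.
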(event Custom|forceUnequipBird
  (params (index :type Integer) (item :type Game%20Item%20Object%20Reference) (dstInventory :type Item%20Inventory%20Object%20Reference) (dstIndex :type Integer))
  ;[0.8878 1 0 0.5] Bird State Manipulation
  (Utilities|And+Branch (== item (Variables|Default|GetequippedBird)) (!= dstInventory (Utilities|GetCharacterInventory "ShortcutBar"))
    (:True
      (Variables|Default|SetequippedBird 0)
      (Variables|Default|SetequippedBirdProfile "")
      (EventDispatchers|UnbindEventfromSignalItemRemoved (Utilities|GetCharacterInventory "ShortcutBar") (delegate Custom|forceUnequipBird)))))

(event Custom|TrackingLoop
  ;[0.05805 1 0.1022] Tracking
  (if (CallFunction|IsValidBirdProfile (Variables|Default|GetequippedBirdProfile))
    (Default|PerformTracking (Utilities|Array|Get(acopy) (stale Custom|toggleTrackingClient _outactors)) self)
    (else
      (CallFunction|ToggleTrackingClient))))

(event Custom|scanInventoryForDocs
  (params (inventory :type Item%20Inventory%20Object%20Reference))
  ;[1 0.03794 0.3524] Document client syncing
  (Variables|Default|SettempCounter 0)
  (while (< (Variables|Default|GettempCounter) (Class|ItemInventory|GetItemCount inventory))
    (CallFunction|ReqUpdateItemDoc (CallFunction|ConstructGameItemRef (Class|ItemInventory|GetItem inventory (Variables|Default|GettempCounter))))
    (Math|Integer|IncrementInt (Variables|Default|GettempCounter))))

(event Custom|OnSignalUpdateStats
  (params (updatedProfile :type STRUCT%20RACO%20Bird%20Profile%20Structure))
  ;[1 1 1] Bird UI Interaction
  (EventDispatchers|BindEventtoBirdProfileCallback (delegate Custom|OnBirdStatsUpdated))
  (CallFunction|ReqUpdateBirdStats (stale Custom|OnBirdProfileReceived itemRef) updatedProfile))

(event Custom|reqUpdateBirdStats
  (params (itemRef :type Game%20Item%20Ref%20Structure) (updatedStats :type STRUCT%20RACO%20Bird%20Profile%20Structure))
  (bind (_travelspeedpoints _carryweightpoints _detectionrangepoints _unspentpoints) (Utilities|Struct|BreakSTRUCT_RACO_BirdProfile updatedStats))
  ;[0.8878 1 0 0.5] Bird State Manipulation
  (bind _item (CallFunction|ResolveGameItemRef itemRef))
  (bind _asbp_base_bird_item (Utilities|Casting|CastToBP_BaseBirdItem _item))
  (bind _structout (Utilities|Struct|SetmembersinSTRUCT_RACO_BirdProfile (Variables|/Game/Mods/RavencrestCouriers/Items/BP_BaseBirdItem.BP_BaseBirdItem_C|GetbirdProfile _asbp_base_bird_item) _travelspeedpoints _carryweightpoints _detectionrangepoints _unspentpoints))
  (bind _output_get (Variables|/Game/Mods/RavencrestCouriers/Items/BP_BaseBirdItem.BP_BaseBirdItem_C|SetbirdProfile _asbp_base_bird_item _structout))
  (CallFunction|TriggerBirdProfileCallback itemRef _output_get))

(event Custom|OnSignalStartEdit
  (params (document :type STRUCT%20RACO%20Document%20Structure))
  ;[0.6069 0.6201 1] Document UI handling
  (Class|GUIModuleController|ActivateModule (Class|GUIModuleController|GetGUIModuleController) (Default|GetDocReadUIModuleName (stale Custom|DocReceivedForReading _asbp_base_document_item)) false false)
  (CallFunction|ClientOpenItemWrite (stale Custom|DocReceivedForReading itemRef)))

(event Custom|clientOpenItemRead
  (params (item :type Game%20Item%20Ref%20Structure))
  ;[0.6069 0.6201 1] Document UI handling
  (EventDispatchers|BindEventtoDocumentCallback (delegate Custom|DocReceivedForReading))
  (CallFunction|ReqGetDocument item))

(event Custom|UpdateBirdDetectionConfig
  (params (config :type STRUCT%20RACO%20Bird%20Detection%20Config%20Structure) (birdPlaceable :type BP%20Base%20Bird%20Placeable%20Object%20Reference))
  ;[1 1 1] Bird UI Interaction
  (Default|UpdateDetectionConfig birdPlaceable config))

(event Custom|reqDocPickUp
  (params (placeable :type BP%20Base%20Document%20Placeable%20Object%20Reference))
  (bind _conancharacter (Utilities|GetConanCharacter))
  (bind _returnvalue (Class|ConanCharacter|GetBackpackInventory _conancharacter))
  ;[1 0.125 0.125] Document Placeable handling
  (bind _returnvalue_2 (Class|ItemInventory|AddItemTemplate _returnvalue (Variables|/Game/Mods/RavencrestCouriers/Items/BP_BaseDocumentPlaceable.BP_BaseDocumentPlaceable_C|GetdocItemTemplateID placeable) -1 "None" 1 false 1.0 -1.0))
  (Variables|/Game/Mods/RavencrestCouriers/Items/BP_BaseDocumentItem.BP_BaseDocumentItem_C|Setdocument (.AsBP%20Base%20Document%20Item (Utilities|Casting|CastToBP_BaseDocumentItem (Class|ItemInventory|GetItem _returnvalue _returnvalue_2))) (Variables|/Game/Mods/RavencrestCouriers/Items/BP_BaseDocumentPlaceable.BP_BaseDocumentPlaceable_C|Getdocument placeable))
  (Actor|DestroyActor placeable))

(event Custom|clientReqCopyDocument
  (params (document :type STRUCT%20RACO%20Document%20Structure) (srcBookItem :type Game%20Item%20Ref%20Structure) (srcBookPlaceable :type BP%20Base%20Document%20Placeable%20Object%20Reference))
  ;[0.569 1 0.2176] Document manipulation
  (bind _returnvalue (Class|GUIModuleController|ActivateModule (Class|GUIModuleController|GetGUIModuleController) "RACO_SelectBook" true false))
  (bind _asw_select_book_view (Utilities|Casting|CastToW_SelectBook_View _returnvalue))
  (Default|InitUI _asw_select_book_view (CallFunction|FindEmptyBooks (Utilities|GetCharacterInventory "Backpack")))
  (EventDispatchers|BindEventtoSignalBookSelected _asw_select_book_view (delegate Custom|OnBookSelected)))

(event Custom|OnBirdStatsUpdated
  (params (itemRef :type Game%20Item%20Ref%20Structure) (birdProfile :type STRUCT%20RACO%20Bird%20Profile%20Structure))
  ;[1 1 1] Bird UI Interaction
  (EventDispatchers|UnbindEventfromBirdProfileCallback (delegate Custom|OnBirdStatsUpdated))
  (Default|InitUI (Variables|Default|GetactiveBirdProfileUI) birdProfile false))

(event Custom|clientOpenBirdProfile
  (params (birdItem :type BP%20Base%20Bird%20Item%20Object%20Reference))
  ;[1 1 1] Bird UI Interaction
  (EventDispatchers|BindEventtoBirdProfileCallback (delegate Custom|OnBirdProfileReceived))
  (CallFunction|ReqGetBirdProfile (CallFunction|ConstructGameItemRef birdItem)))

(event Custom|OnSignalCopyDocument
  (params (document :type STRUCT%20RACO%20Document%20Structure))
  ;[0.6069 0.6201 1] Document UI handling
  (CallFunction|ClientReqCopyDocument document (stale Custom|DocReceivedForReading itemRef)))

(event Custom|reqGetDocument
  (params (itemRef :type Game%20Item%20Ref%20Structure))
  ;[0.569 1 0.2176] Document manipulation
  (bind _item (CallFunction|ResolveGameItemRef itemRef))
  (bind _asbp_base_document_item (Utilities|Casting|CastToBP_BaseDocumentItem _item))
  (CallFunction|TriggerDocumentCallback itemRef (Variables|/Game/Mods/RavencrestCouriers/Items/BP_BaseDocumentItem.BP_BaseDocumentItem_C|Getdocument _asbp_base_document_item)))

(event Custom|OnBirdProfileUIClosing
  (params (window :type Window%20Root%20Object%20Reference))
  ;[1 1 1] Bird UI Interaction
  (Variables|Default|SetactiveBirdProfileUI 0)
  (CallFunction|DisposeBirdPreview))

(event Custom|clientOpenItemWrite
  (params (item :type Game%20Item%20Ref%20Structure))
  ;[0.6069 0.6201 1] Document UI handling
  (EventDispatchers|BindEventtoDocumentCallback (delegate Custom|DocReceivedForWriting))
  (CallFunction|ReqGetDocument item))

(event Custom|DoDownloadBook
  (params (bookId :type String))
  (bind _returnvalue (Utilities|String|MakeLiteralString "{\"uuid\":\"4c52d6b7-51bb-4308-b2a8-d49504f59044\",
\"title\":\"My Private Journal\",\"author\":\"Anonymous\",
\"create_date\":\"2023-06-13T20:42:03.142Z\",
\"testQuote\": \"A wise man once said: \\\"Hello World\\\"\",
\"update_date\":\"2023-06-13T22:31:32.033Z\",
}"))
  (bind _datamap (CallFunction|ParseSimpleJSON _returnvalue))
  ;[0.3327 0.1928 1] Athenaeum
  (bind _keys (Utilities|Map|Keys _datamap))
  (for _array_element _keys
    (Development|PrintString (Utilities|String|Append _array_element " = " (.Value (Utilities|Map|Find _datamap _array_element))) true true "(R=0.000000,G=0.660000,B=1.000000,A=1.000000)" 6.0)))

(event Custom|reqStartPlacement
  (params (itemRef :type Game%20Item%20Ref%20Structure))
  (bind _conancharacter (Utilities|GetConanCharacter))
  ;[0.8878 1 0 0.5] Bird State Manipulation
  (bind _item (CallFunction|ResolveGameItemRef itemRef))
  (bind _asbp_base_bird_item (Utilities|Casting|CastToBP_BaseBirdItem _item))
  (Variables|Default|SetbirdProfileBeingPlaced (Variables|/Game/Mods/RavencrestCouriers/Items/BP_BaseBirdItem.BP_BaseBirdItem_C|GetbirdProfile _asbp_base_bird_item))
  (Default|TriggerStartPlacement _asbp_base_bird_item _conancharacter _conancharacter))

(event Custom|notifyItemBeingPlaced
  (params (item :type Game%20Item%20Ref%20Structure))
  ;[1 0.125 0.125] Document Placeable handling
  (bind _item (CallFunction|ResolveGameItemRef item))
  (bind _asbp_base_document_item (Utilities|Casting|CastToBP_BaseDocumentItem _item))
  (Variables|Default|SetdocBeingPlaced (Variables|/Game/Mods/RavencrestCouriers/Items/BP_BaseDocumentItem.BP_BaseDocumentItem_C|Getdocument _asbp_base_document_item))
  (Variables|Default|SetdocTemplateID (Variables|/Script/ConanSandbox.GameItem|GetTemplateID _item)))

(event Custom|clientOpenBirdProfile2
  (params (profile :type STRUCT%20RACO%20Bird%20Profile%20Structure))
  ;[1 1 1] Bird UI Interaction
  (CallFunction|PrepareBirdPreview (CallFunction|GetBirdTypebyID (Utilities|Struct|BreakSTRUCT_RACO_BirdProfile profile)))
  (bind _windowroot (|GUIModuleControllerActivate (Class|GUIModuleController|GetGUIModuleController) "RACO_ViewBirdProfile" true false)
    (:OnActivate
      (bind _output_get (Variables|Default|SetactiveBirdProfileUI (.AsW%20Bird%20Profile%20View (Utilities|Casting|CastToW_BirdProfile_View _windowroot))))
      (Default|InitUI _output_get profile true)
      (EventDispatchers|BindEventtoSignalClosing _windowroot (delegate Custom|OnBirdProfileUIClosing)))))

(event Custom|OnSignalPlaceBird
  (bind _conancharacter (Utilities|GetConanCharacter))
  ;[1 1 1] Bird UI Interaction
  (CallFunction|ReqStartPlacement (stale Custom|OnBirdProfileReceived itemRef))
  (bind _item (CallFunction|ResolveGameItemRef (stale Custom|OnBirdProfileReceived itemRef)))
  (Default|TriggerStartPlacement (.AsBP%20Base%20Bird%20Item (Utilities|Casting|CastToBP_BaseBirdItem _item)) _conancharacter _conancharacter))

(event Custom|OnSignalEquipBird
  ;[1 1 1] Bird UI Interaction
  (CallFunction|ReqEquipBird (stale Custom|OnBirdProfileReceived itemRef)))

(event Custom|notifyItemPlacementDone
  (bind _returnvalue (Components|GetOwner))
  (bind _returnvalue_2 (Actor|GetComponentbyClass _returnvalue "/Game/Systems/Building/BP_BuildSystem_v2.BP_BuildSystem_v2_C"))
  ;[1 0.125 0.125] Document Placeable handling
  (if (Variables|/Script/ConanSandbox.BuildSystemComponent|GetIsBuilding _returnvalue_2)
    (Class|BuildSystemComponent|StopBuilding _returnvalue_2)))

(event Custom|reqEquipBird
  (params (itemRef :type Game%20Item%20Ref%20Structure))
  (bind _inventory (Utilities|GetCharacterInventory "ShortcutBar"))
  ;[0.8878 1 0 0.5] Bird State Manipulation
  (bind _item (CallFunction|ResolveGameItemRef itemRef))
  (bind _asbp_base_bird_item (Utilities|Casting|CastToBP_BaseBirdItem _item))
  (if (== _asbp_base_bird_item (Variables|Default|GetequippedBird))
    (Variables|Default|SetequippedBird 0)
    (Variables|Default|SetequippedBirdProfile "")
    (EventDispatchers|UnbindEventfromSignalItemRemoved _inventory (delegate Custom|forceUnequipBird))
    (elif (== (Utilities|GetCharacterInventory "ShortcutBar") (Class|GameItem|GetOwnerInventory _asbp_base_bird_item))
      (bind _output_get (Variables|Default|SetequippedBird _asbp_base_bird_item))
      (Variables|Default|SetequippedBirdProfile (Variables|/Game/Mods/RavencrestCouriers/Items/BP_BaseBirdItem.BP_BaseBirdItem_C|GetbirdProfile _output_get))
      (EventDispatchers|BindEventtoSignalItemRemoved _inventory (delegate Custom|forceUnequipBird)))))

(event Custom|clientOpenBirdDetectionConfig
  (params (birdPlaceable :type BP%20Base%20Bird%20Placeable%20Object%20Reference))
  ;[1 1 1] Bird UI Interaction
  (bind _windowroot (|GUIModuleControllerActivate (Class|GUIModuleController|GetGUIModuleController) "RACO_ViewBirdDetectionConfig" true false)
    (:OnActivate
      (Default|InitUI (.AsW%20Bird%20Detection%20Config%20View (Utilities|Casting|CastToW_BirdDetectionConfig_View _windowroot)) (Variables|/Game/Mods/RavencrestCouriers/Items/BP_BaseBirdPlaceable.BP_BaseBirdPlaceable_C|GetbirdProfile birdPlaceable) (Variables|/Game/Mods/RavencrestCouriers/Items/BP_BaseBirdPlaceable.BP_BaseBirdPlaceable_C|GetbirdDetectionConfig birdPlaceable))
      (EventDispatchers|BindEventtoSignalUpdateConfig (.AsW%20Bird%20Detection%20Config%20View (Utilities|Casting|CastToW_BirdDetectionConfig_View _windowroot)) (delegate Custom|OnSignalUpdateConfig)))))

(event Custom|clientOpenPlaceableRead
  (params (placeable :type Actor%20Object%20Reference) (document :type STRUCT%20RACO%20Document%20Structure))
  ;[0.6069 0.6201 1] Document UI handling
  (bind _asbp_base_document_placeable (Utilities|Casting|CastToBP_BaseDocumentPlaceable placeable))
  (bind _returnvalue (Class|GUIModuleController|ActivateModule (Class|GUIModuleController|GetGUIModuleController) (Default|GetDocReadUIModuleName _asbp_base_document_placeable) true false))
  (bind _asw_raco_base_read_ui (Utilities|Casting|CastToW_RACO_BaseReadUI _returnvalue))
  (Default|UpdateDocument _asw_raco_base_read_ui document false)
  (EventDispatchers|BindEventtoSignalCopyDocument _asw_raco_base_read_ui (delegate Custom|OnSignalCopyDoc)))

(event Custom|clientUpdateItemDoc
  (params (item :type Game%20Item%20Ref%20Structure) (doc :type STRUCT%20RACO%20Document%20Structure))
  ;[1 0.03794 0.3524] Document client syncing
  (bind _item (CallFunction|ResolveGameItemRef item))
  (bind _asbp_base_document_item (Utilities|Casting|CastToBP_BaseDocumentItem _item))
  (Variables|/Game/Mods/RavencrestCouriers/Items/BP_BaseDocumentItem.BP_BaseDocumentItem_C|Setdocument _asbp_base_document_item doc))

(event Custom|LoopBirdRandomAnimation
  (bind _equippedbirdprofile (Variables|Default|GetequippedBirdProfile))
  (bind _birdtypeid (Utilities|Struct|BreakSTRUCT_RACO_BirdProfile _equippedbirdprofile))
  ;[0.8878 1 0 0.5] Bird State Manipulation
  (if (Math|Boolean|NORBoolean (Networking|IsDedicatedServer) (Utilities|Array|IsEmpty (Utilities|String|ToString(Name) _birdtypeid)))
    (bind _animlength (CallFunction|PlayRandomBirdAnimation (Variables|Default|GetequippedBirdMesh) _birdtypeid))
    (Utilities|FlowControl|Delay (+ _animlength (Math|Random|RandomFloatinRange 2.0 5.0)))
    (CallFunction|LoopBirdRandomAnimation)))

(event Custom|toggleTrackingClient
  ;[0.05805 1 0.1022] Tracking
  (if (Utilities|Struct|BreakSTRUCT_RACO_ServerSettings (CallFunction|GetServerSettings))
    (bind _output_get (Variables|Default|SetisTrackingActive (not (Class|GUIModuleController|IsModuleActive (Class|GUIModuleController|GetGUIModuleController) "RACO_Tracking_HUD"))))
    (bind _returnvalue (Class|GUIModuleController|ActivateModule (Class|GUIModuleController|GetGUIModuleController) "RACO_Tracking_HUD" _output_get false))
    (if (Variables|Default|GetisTrackingActive)
      (bind _outactors (Actor|GetAllActorsOfClass "/Game/Mods/RavencrestCouriers/System/BP_RACO_TrackingSystem.BP_RACO_TrackingSystem_C"))
      (Default|InitHUD (.AsW%20Tracking%20HUD (Utilities|Casting|CastToW_Tracking_HUD _returnvalue)) (Utilities|Array|Get(acopy) _outactors))
      (bind _returnvalue_2 (Utilities|Time|SetTimerbyEvent (delegate Custom|TrackingLoop) 5.0 true))
      (Variables|Default|SettrackingTimer _returnvalue_2)
      (else
        (Utilities|Time|ClearandInvalidateTimerbyHandle (Variables|Default|GettrackingTimer))))
    (else
      (bind _returnvalue_3 (Class|MessageBoxWidget|CreateMessageBox (Components|GetOwner) "OK" "Tracking Disabled" "Bird Tracking has been disabled on this server."))
      (Class|MessageBoxWidget|ShowMessageBox _returnvalue_3 0 1001))))

(event Custom|OnBirdToggleTracking
  ;[1 1 1] Bird UI Interaction
  (CallFunction|ToggleTrackingClient))

(event Custom|DocReceivedForReading
  (params (itemRef :type Game%20Item%20Ref%20Structure) (document :type STRUCT%20RACO%20Document%20Structure))
  ;[0.6069 0.6201 1] Document UI handling
  (EventDispatchers|UnbindEventfromDocumentCallback (delegate Custom|DocReceivedForReading))
  (if (CallFunction|IsNewDocument document)
    (CallFunction|ClientOpenItemWrite itemRef)
    (else
      (bind _item (CallFunction|ResolveGameItemRef itemRef))
      (bind _asbp_base_document_item (Utilities|Casting|CastToBP_BaseDocumentItem _item))
      (bind _returnvalue (Class|GUIModuleController|ActivateModule (Class|GUIModuleController|GetGUIModuleController) (Default|GetDocReadUIModuleName _asbp_base_document_item) true false))
      (bind _asw_raco_base_read_ui (Utilities|Casting|CastToW_RACO_BaseReadUI _returnvalue))
      (Default|UpdateDocument _asw_raco_base_read_ui document true)
      (EventDispatchers|BindEventtoSignalEditDocument _asw_raco_base_read_ui (delegate Custom|OnSignalStartEdit))
      (EventDispatchers|BindEventtoSignalCopyDocument _asw_raco_base_read_ui (delegate Custom|OnSignalCopyDocument))
      (EventDispatchers|BindEventtoSignalBreakSeal _asw_raco_base_read_ui (delegate Custom|OnSignalBreakSeal)))))

(event Custom|OnSignalChangeName
  (params (newName :type String))
  ;[1 1 1] Bird UI Interaction
  (EventDispatchers|BindEventtoBirdProfileCallback (delegate Custom|OnBirdNameChanged))
  (CallFunction|ReqChangeBirdName (stale Custom|OnBirdProfileReceived itemRef) newName))

(event Custom|reqGetBirdProfile
  (params (itemRef :type Game%20Item%20Ref%20Structure))
  ;[0.8878 1 0 0.5] Bird State Manipulation
  (bind _item (CallFunction|ResolveGameItemRef itemRef))
  (bind _asbp_base_bird_item (Utilities|Casting|CastToBP_BaseBirdItem _item))
  (if (CallFunction|IsValidBirdProfile (Variables|/Game/Mods/RavencrestCouriers/Items/BP_BaseBirdItem.BP_BaseBirdItem_C|GetbirdProfile _asbp_base_bird_item))
    (CallFunction|TriggerBirdProfileCallback itemRef (Variables|/Game/Mods/RavencrestCouriers/Items/BP_BaseBirdItem.BP_BaseBirdItem_C|GetbirdProfile _asbp_base_bird_item))
    (else
      (bind _newprofile (CallFunction|CreateNewBirdProfile (Variables|/Game/Mods/RavencrestCouriers/Items/BP_BaseBirdItem.BP_BaseBirdItem_C|GetbirdTypeID _asbp_base_bird_item)))
      (bind _output_get (Variables|/Game/Mods/RavencrestCouriers/Items/BP_BaseBirdItem.BP_BaseBirdItem_C|SetbirdProfile _asbp_base_bird_item _newprofile))
      (CallFunction|TriggerBirdProfileCallback itemRef _output_get))))

(event Custom|OnBirdProfileReceived
  (params (itemRef :type Game%20Item%20Ref%20Structure) (birdProfile :type STRUCT%20RACO%20Bird%20Profile%20Structure))
  ;[1 1 1] Bird UI Interaction
  (EventDispatchers|UnbindEventfromBirdProfileCallback (delegate Custom|OnBirdProfileReceived))
  (CallFunction|PrepareBirdPreview (CallFunction|GetBirdTypebyID (Utilities|Struct|BreakSTRUCT_RACO_BirdProfile birdProfile)))
  (bind _windowroot (|GUIModuleControllerActivate (Class|GUIModuleController|GetGUIModuleController) "RACO_ViewBirdProfile" true false)
    (:OnActivate
      (bind _output_get (Variables|Default|SetactiveBirdProfileUI (.AsW%20Bird%20Profile%20View (Utilities|Casting|CastToW_BirdProfile_View _windowroot))))
      (Default|InitUI _output_get birdProfile false)
      (EventDispatchers|BindEventtoSignalEquipBird (Variables|Default|GetactiveBirdProfileUI) (delegate Custom|OnSignalEquipBird))
      (EventDispatchers|BindEventtoSignalPlaceBird (Variables|Default|GetactiveBirdProfileUI) (delegate Custom|OnSignalPlaceBird))
      (EventDispatchers|BindEventtoSignalChangeBirdName (Variables|Default|GetactiveBirdProfileUI) (delegate Custom|OnSignalChangeName))
      (EventDispatchers|BindEventtoSignalUpdateStats (Variables|Default|GetactiveBirdProfileUI) (delegate Custom|OnSignalUpdateStats))
      (EventDispatchers|BindEventtoSignalClosing (Variables|Default|GetactiveBirdProfileUI) (delegate Custom|OnBirdProfileUIClosing))
      (EventDispatchers|BindEventtoSignalToggleTracking (Variables|Default|GetactiveBirdProfileUI) (delegate Custom|OnBirdToggleTracking)))))

(event Custom|reqChangeBirdName
  (params (itemRef :type Game%20Item%20Ref%20Structure) (newName :type String))
  ;[0.8878 1 0 0.5] Bird State Manipulation
  (bind _item (CallFunction|ResolveGameItemRef itemRef))
  (bind _asbp_base_bird_item (Utilities|Casting|CastToBP_BaseBirdItem _item))
  (bind _structout (Utilities|Struct|SetmembersinSTRUCT_RACO_BirdProfile (Variables|/Game/Mods/RavencrestCouriers/Items/BP_BaseBirdItem.BP_BaseBirdItem_C|GetbirdProfile _asbp_base_bird_item) newName))
  (bind _output_get (Variables|/Game/Mods/RavencrestCouriers/Items/BP_BaseBirdItem.BP_BaseBirdItem_C|SetbirdProfile _asbp_base_bird_item _structout))
  (CallFunction|TriggerBirdProfileCallback itemRef _output_get))

(event Custom|triggerBirdProfileCallback
  (params (itemRef :type Game%20Item%20Ref%20Structure) (birdProfile :type STRUCT%20RACO%20Bird%20Profile%20Structure))
  ;[0.8878 1 0 0.5] Bird State Manipulation
  (Default|CallBirdProfileCallback itemRef birdProfile))

(event Custom|triggerDocumentCallback
  (params (itemRef :type Game%20Item%20Ref%20Structure) (document :type STRUCT%20RACO%20Document%20Structure))
  ;[0.569 1 0.2176] Document manipulation
  (Default|CallDocumentCallback itemRef document))

(event Custom|OnSignalBreakSeal
  (params (document :type STRUCT%20RACO%20Document%20Structure))
  ;[0.6069 0.6201 1] Document UI handling
  (EventDispatchers|BindEventtoDocumentCallback (delegate Custom|OnSealBroken))
  (CallFunction|ReqBreakSeal (stale Custom|DocReceivedForReading itemRef) document))

(event Custom|InitAthenaeumPanel
  (params (panel :type W%20Athenaeum%20Panel%20Object%20Reference))
  ;[0.3327 0.1928 1] Athenaeum
  (EventDispatchers|BindEventtoSignalDownloadBook panel (delegate Custom|DoDownloadBook)))

(event Custom|reqUpdateItemDoc
  (params (item :type Game%20Item%20Ref%20Structure))
  ;[1 0.03794 0.3524] Document client syncing
  (bind _item (CallFunction|ResolveGameItemRef item))
  (bind _asbp_base_document_item (Utilities|Casting|CastToBP_BaseDocumentItem _item))
  (CallFunction|ClientUpdateItemDoc (CallFunction|ConstructGameItemRef _asbp_base_document_item) (Variables|/Game/Mods/RavencrestCouriers/Items/BP_BaseDocumentItem.BP_BaseDocumentItem_C|Getdocument _asbp_base_document_item)))

(event Custom|DocReceivedForWriting
  (params (itemRef :type Game%20Item%20Ref%20Structure) (document :type STRUCT%20RACO%20Document%20Structure))
  ;[0.6069 0.6201 1] Document UI handling
  (EventDispatchers|UnbindEventfromDocumentCallback (delegate Custom|DocReceivedForWriting))
  (bind _item (CallFunction|ResolveGameItemRef itemRef))
  (bind _asbp_base_document_item (Utilities|Casting|CastToBP_BaseDocumentItem _item))
  (bind _returnvalue (Class|GUIModuleController|ActivateModule (Class|GUIModuleController|GetGUIModuleController) (Default|GetDocWriteUIModuleName _asbp_base_document_item) true false))
  (bind _asw_raco_base_write_ui (Utilities|Casting|CastToW_RACO_BaseWriteUI _returnvalue))
  (bind _structout (Utilities|Struct|SetmembersinSTRUCT_RACO_Document document (CallFunction|GetAuthorName)))
  (Default|InitDocument _asw_raco_base_write_ui _structout)
  (EventDispatchers|BindEventtoSignalSaveDocument _asw_raco_base_write_ui (delegate Custom|OnSignalSaveDoc)))

(event Custom|reqChangeName
  (params (placeable :type BP%20Placeable%20Item%20Container%20Object%20Reference) (newName :type Text))
  ;[1 0.125 0.125] Document Placeable handling
  (Class|BuildableBase|SetBuildableName placeable newName)
  (Class|PersistenceComponent|SetDirty (Variables|/Game/Systems/Building/Placeables/BP_Master_Placeables.BP_Master_Placeables_C|GetConanBuildingPersistence placeable) true 3.0))

(event Custom|reqSaveDocument
  (params (itemRef :type Game%20Item%20Ref%20Structure) (document :type STRUCT%20RACO%20Document%20Structure))
  ;[0.569 1 0.2176] Document manipulation
  (bind _item (CallFunction|ResolveGameItemRef itemRef))
  (bind _asbp_base_document_item (Utilities|Casting|CastToBP_BaseDocumentItem _item))
  (if (CallFunction|IsNewDocument document)
    (bind _structout (Utilities|Struct|SetmembersinSTRUCT_RACO_Document document (Guid|ToString(Guid) (Guid|NewGuid))))
    (bind _output_get (Variables|/Game/Mods/RavencrestCouriers/Items/BP_BaseDocumentItem.BP_BaseDocumentItem_C|Setdocument _asbp_base_document_item _structout))
    (CallFunction|TriggerDocumentCallback itemRef _output_get)
    (CallFunction|ClientUpdateItemDoc itemRef _output_get)
    (else
      (bind _output_get_2 (Variables|/Game/Mods/RavencrestCouriers/Items/BP_BaseDocumentItem.BP_BaseDocumentItem_C|Setdocument _asbp_base_document_item document))
      (CallFunction|TriggerDocumentCallback itemRef _output_get_2)
      (CallFunction|ClientUpdateItemDoc itemRef _output_get_2))))

(event Custom|InitInventoryDocSync
  (bind _inventory (Utilities|GetCharacterInventory "ShortcutBar"))
  (bind _inventory_2 (Utilities|GetCharacterInventory "Backpack"))
  ;[1 0.03794 0.3524] Document client syncing
  (if (Networking|IsServer)
    (EventDispatchers|BindEventtoSignalItemAdded _inventory_2 (delegate Custom|OnItemAdded))
    (CallFunction|ScanInventoryforDocs _inventory_2)
    (EventDispatchers|BindEventtoSignalItemAdded _inventory (delegate Custom|OnItemAdded))
    (CallFunction|ScanInventoryforDocs _inventory)))

(event Custom|reqPickupBird
  (params (birdPlaceable :type BP%20Base%20Bird%20Placeable%20Object%20Reference))
  (bind _conancharacter (Utilities|GetConanCharacter))
  (bind _returnvalue (Class|ConanCharacter|GetBackpackInventory _conancharacter))
  ;[0.8878 1 0 0.5] Bird State Manipulation
  (Utilities|FlowControl|Sequence
    (:then_0
      (bind _returnvalue_2 (Class|ItemInventory|AddItemTemplate _returnvalue (Variables|/Script/ConanSandbox.BuildableBase|GetSourceItemTemplateID birdPlaceable) -1 "None" 1 false 1.0 -1.0))
      (Variables|/Game/Mods/RavencrestCouriers/Items/BP_BaseBirdItem.BP_BaseBirdItem_C|SetbirdProfile (.AsBP%20Base%20Bird%20Item (Utilities|Casting|CastToBP_BaseBirdItem (Class|ItemInventory|GetItem _returnvalue _returnvalue_2))) (Variables|/Game/Mods/RavencrestCouriers/Items/BP_BaseBirdPlaceable.BP_BaseBirdPlaceable_C|GetbirdProfile birdPlaceable)))
    (:then_1
      (Actor|DestroyActor birdPlaceable))))

(event Custom|OnSignalSaveDoc
  (params (document :type STRUCT%20RACO%20Document%20Structure))
  ;[0.6069 0.6201 1] Document UI handling
  (CallFunction|ReqSaveDocument (stale Custom|DocReceivedForWriting itemRef) document))

(event Custom|OnBirdNameChanged
  (params (itemRef :type Game%20Item%20Ref%20Structure) (birdProfile :type STRUCT%20RACO%20Bird%20Profile%20Structure))
  ;[1 1 1] Bird UI Interaction
  (EventDispatchers|UnbindEventfromBirdProfileCallback (delegate Custom|OnBirdNameChanged))
  (Default|InitUI (Variables|Default|GetactiveBirdProfileUI) birdProfile false))

(event Custom|OnSignalCopyDoc
  (params (document :type STRUCT%20RACO%20Document%20Structure))
  ;[0.6069 0.6201 1] Document UI handling
  (CallFunction|ClientReqCopyDocument :document document :srcBookPlaceable (stale Custom|clientOpenPlaceableRead _asbp_base_document_placeable)))

(event Custom|OnBookSelected
  (params (selectedBook :type Game%20Item%20Ref%20Structure))
  ;[0.569 1 0.2176] Document manipulation
  (CallFunction|ReqCopyDocument (stale Custom|clientReqCopyDocument document) selectedBook))

(event Custom|OnSignalUpdateConfig
  (params (updatedConfig :type STRUCT%20RACO%20Bird%20Detection%20Config%20Structure))
  ;[1 1 1] Bird UI Interaction
  (CallFunction|UpdateBirdDetectionConfig updatedConfig (stale Custom|clientOpenBirdDetectionConfig birdPlaceable)))

(event Custom|reqCopyDocument
  (params (document :type STRUCT%20RACO%20Document%20Structure) (destBookItem :type Game%20Item%20Ref%20Structure))
  ;[0.569 1 0.2176] Document manipulation
  (bind _item (CallFunction|ResolveGameItemRef destBookItem))
  (if (.bSuccess (Utilities|Casting|CastToBP_BaseDocumentItem _item))
    (bind _documentcopy (CallFunction|DuplicateDocument document))
    (bind _output_get (Variables|/Game/Mods/RavencrestCouriers/Items/BP_BaseDocumentItem.BP_BaseDocumentItem_C|Setdocument (.AsBP%20Base%20Document%20Item (Utilities|Casting|CastToBP_BaseDocumentItem _item)) _documentcopy))
    (Class|ConanCharacter|ClientHUDShowNotification (Utilities|GetConanCharacter) (Utilities|Text|MakeLiteralText "You copied the contents of the book") true true)
    (CallFunction|ClientUpdateItemDoc destBookItem _output_get)))

(event Custom|reqBreakSeal
  (params (itemRef :type Game%20Item%20Ref%20Structure) (document :type STRUCT%20RACO%20Document%20Structure))
  ;[0.569 1 0.2176] Document manipulation
  (bind _item (CallFunction|ResolveGameItemRef itemRef))
  (bind _asbp_base_document_item (Utilities|Casting|CastToBP_BaseDocumentItem _item))
  (if (Utilities|Struct|BreakSTRUCT_RACO_Document document)
    (bind _structout (Utilities|Struct|SetmembersinSTRUCT_RACO_Document document false))
    (bind _output_get (Variables|/Game/Mods/RavencrestCouriers/Items/BP_BaseDocumentItem.BP_BaseDocumentItem_C|Setdocument _asbp_base_document_item _structout))
    (CallFunction|TriggerDocumentCallback itemRef _output_get)))

(event Custom|OnItemAdded
  (params (index :type Integer) (item :type Game%20Item%20Object%20Reference) (srcInventory :type Item%20Inventory%20Object%20Reference) (srcIndex :type Integer))
  ;[1 0.03794 0.3524] Document client syncing
  (CallFunction|ReqUpdateItemDoc (CallFunction|ConstructGameItemRef item)))

(event Custom|OnSealBroken
  (params (itemRef :type Game%20Item%20Ref%20Structure) (document :type STRUCT%20RACO%20Document%20Structure))
  ;[0.6069 0.6201 1] Document UI handling
  (EventDispatchers|UnbindEventfromDocumentCallback (delegate Custom|OnSealBroken))
  (Default|UpdateDocument (stale Custom|DocReceivedForReading _asw_raco_base_read_ui) document true))

(event EventBeginPlay
  (CallFunction|InitInventoryDocSync)
  (if (not (Networking|IsServer))
    (CallFunction|OnRepEquippedBirdProfile)))

(fn GetAuthorName
  (bind _conancharacter (Utilities|GetConanCharacter))
  (bind _returnvalue (Class|ConanCharacter|GetGuild _conancharacter))
  (LocalVariables|SetauthorName (Class|ConanCharacter|GetCharacterName (Utilities|GetConanCharacter)))
  (Utilities|FlowControl|Sequence
    (:then_0
      (Utilities|IsValid _returnvalue
        (:Is%20Valid
          (LocalVariables|SetauthorName (Utilities|String|Append (LocalVariables|GetauthorName) " of " (Class|Guild|GetGuildName _returnvalue))))))
    (:then_1
      (return (LocalVariables|GetauthorName)))))

(fn PrepareBirdPreview
  (params (birdType :type STRUCT%20RACO%20Bird%20Type%20Structure))
  (bind (_skeletalmesh _transform _idleanimations) (Utilities|Struct|BreakSTRUCT_RACO_BirdType birdType))
  (Utilities|FlowControl|Sequence
    (:then_0
      (Utilities|IsValid (Variables|Default|GetbirdPreviewRoom)
        (:Is%20Not%20Valid
          (bind _returnvalue (Game|SpawnActorfromClass "/Game/Mods/RavencrestCouriers/UI/bird_preview/BP_RACO_PreviewRoom.BP_RACO_PreviewRoom_C" (Math|Conversions|ToTransform(Vector) "0, 0,-15000.000000") "Undefined" "OverrideRootScale" (Components|GetOwner) 0))
          (Variables|Default|SetbirdPreviewRoom _returnvalue))))
    (:then_1
      (Transformation|SetRelativeTransform (Variables|/Game/Mods/RavencrestCouriers/UI/bird_preview/BP_RACO_PreviewRoom.BP_RACO_PreviewRoom_C|GetSkeletalMesh (Variables|Default|GetbirdPreviewRoom)) _transform false false)
      (Components|SkinnedMesh|SetSkinnedAssetandUpdate (Variables|/Game/Mods/RavencrestCouriers/UI/bird_preview/BP_RACO_PreviewRoom.BP_RACO_PreviewRoom_C|GetSkeletalMesh (Variables|Default|GetbirdPreviewRoom)) _skeletalmesh true)
      (Components|Animation|PlayAnimation (Variables|/Game/Mods/RavencrestCouriers/UI/bird_preview/BP_RACO_PreviewRoom.BP_RACO_PreviewRoom_C|GetSkeletalMesh (Variables|Default|GetbirdPreviewRoom)) (Utilities|Array|Get(acopy) _idleanimations) true))))

(fn OnRepEquippedBirdProfile
  (bind _equippedbirdprofile (Variables|Default|GetequippedBirdProfile))
  (bind _birdtypeid (Utilities|Struct|BreakSTRUCT_RACO_BirdProfile _equippedbirdprofile))
  (bind _birdtype (CallFunction|GetBirdTypebyID _birdtypeid))
  (bind (_skeletalmesh _transform) (Utilities|Struct|BreakSTRUCT_RACO_BirdType _birdtype))
  (Utilities|FlowControl|Sequence
    (:then_0
      (bind _output_get (LocalVariables|Setcharacter (Utilities|GetConanCharacter)))
      (Utilities|IsValid _output_get
        (:Is%20Valid
          (LocalVariables|SetcharacterGender (Class|ConanCharacter|GetIntStat _output_get "Gender" "Full")))))
    (:then_1
      (Utilities|IsValid (Variables|Default|GetequippedBirdMesh)
        (:Is%20Not%20Valid
          (bind _returnvalue (Class|CharacterFunctionLibrary|AddSkeletalMeshComponent (LocalVariables|Getcharacter) true (Utilities|Select :Index (- (LocalVariables|GetcharacterGender) 1) :Option%200 (LocalVariables|GetmaleTransform) :Option%201 (LocalVariables|GetfemaleTransform)) "/Script/Engine.SkeletalMeshComponent"))
          (bind _output_get_2 (Variables|Default|SetequippedBirdMesh _returnvalue))
          (Transformation|AttachComponentToComponent _output_get_2 (Variables|/Script/Engine.Character|GetMesh (LocalVariables|Getcharacter)) "b_R_clavicle" "KeepRelative" "KeepRelative" "KeepRelative" true))))
    (:then_2
      (if (CallFunction|IsValidBirdProfile _equippedbirdprofile)
        (Transformation|SetRelativeTransform (Variables|Default|GetequippedBirdMesh) (Math|Transform|ComposeTransforms (Utilities|Select :Index (- (LocalVariables|GetcharacterGender) 1) :Option%200 (LocalVariables|GetmaleTransform) :Option%201 (LocalVariables|GetfemaleTransform)) _transform) false false)
        (Components|SkinnedMesh|SetSkinnedAssetandUpdate (Variables|Default|GetequippedBirdMesh) _skeletalmesh true)
        (CallFunction|LoopBirdRandomAnimation)
        (else
          (Components|SkinnedMesh|SetSkinnedAssetandUpdate (Variables|Default|GetequippedBirdMesh) 0 true))))))

(fn IsBirdEquipped
  (params (profileGUID :type String))
  (return (Utilities|Enum|Equal(Enum) profileGUID (Utilities|Struct|BreakSTRUCT_RACO_BirdProfile (Variables|Default|GetequippedBirdProfile)))))

(fn DisposeBirdPreview
  (Utilities|IsValid (Variables|Default|GetbirdPreviewRoom)
    (:Is%20Valid
      (Actor|DestroyActor (Variables|Default|GetbirdPreviewRoom))
      (Variables|Default|SetbirdPreviewRoom 0))))